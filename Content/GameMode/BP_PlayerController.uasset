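; Player controller that lets the player switch possession between the BP_Player character and a DefaultPawn using numpad keys.
; BeginPlay caches the first BP_Player, BP_PossessPawn and DefaultPawn found, though the BP_PossessPawn reference is unused here.
; NumPad 6 flip-flops possession, hiding the cursor for BP_Player and enabling cursor, click and hover events for DefaultPawn.
; NumPad 5 possesses BP_Player, unpossesses after a short delay, then enables those cursor settings.
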(event EventBeginPlay
  (bind _outactors (Actor|GetAllActorsOfClass "/Game/Player/BP_Player.BP_Player_C"))
  (Variables|Default|SetPossessPawn (Utilities|Array|Get(acopy) _outactors))
  (bind _outactors_2 (Actor|GetAllActorsOfClass "/Game/Demo/BP_PossessPawn.BP_PossessPawn_C"))
  (Variables|Default|SetAnotherPawn (Utilities|Array|Get(acopy) _outactors_2))
  (bind _outactors_3 (Actor|GetAllActorsOfClass "/Script/Engine.DefaultPawn"))
  (Variables|Default|SetDefaultPawn (Utilities|Array|Get(acopy) _outactors_3)))

(event EventTick
  (params (DeltaSeconds :type Float%20%28single-precision%29)))

(event Input|KeyboardEvents|NumPadSix
  (params (Key :type Key%20Structure :default "None"))
  (:Pressed
    (Utilities|FlowControl|FlipFlop
      (:A
        (Pawn|Possess (Variables|Default|GetPossessPawn))
        (Variables|Default|SetbShowMouseCursor false)
        (Variables|Default|SetbEnableMouseOverEvents false)
        (Variables|Default|SetbEnableClickEvents false))
      (:B
        (Pawn|Possess (Variables|Default|GetDefaultPawn))
        (Variables|Default|SetbShowMouseCursor true)
        (Variables|Default|SetbEnableMouseOverEvents true)
        (Variables|Default|SetbEnableClickEvents true)))))

(event Input|KeyboardEvents|NumPadFive
  (params (Key :type Key%20Structure :default "None"))
  (:Pressed
    (Pawn|Possess (Variables|Default|GetPossessPawn))
    (Utilities|FlowControl|Delay 0.2)
    (Pawn|UnPossess)
    (Variables|Default|SetbShowMouseCursor true)
    (Variables|Default|SetbEnableMouseOverEvents true)
    (Variables|Default|SetbEnableClickEvents true)))

(fn ConstructionScript)