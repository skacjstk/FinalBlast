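; AI controller for ranged enemies that, on possession, runs the behavior tree stored on its BP_Enemy_AI pawn.
; Perception updates scan currently perceived actors, writing a sensed player to PlayerKey or a "Grenade Noise" stimulus's location and flag to the blackboard.
; The first such match breaks the search through a custom event.
; PlayerKey clears when no player is found, and the noise flag clears when neither is found.
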(event OnPerceptionUpdated(AIPerception)
  (params (UpdatedActors :type Array%20of%20Actor%20Object%20References))
  (Variables|Default|SetIsFindPlayer false)
  (Variables|Default|SetIsNoiseHearing false)
  (Utilities|FlowControl|Sequence
    (:then_0
      (bind _array_element (Utilities|Array|ForEachLoopwithBreak (Class|AIPerceptionComponent|GetCurrentlyPerceivedActors (Variables|Default|GetAIPerception)))
        (:LoopBody
          (bind _info (Class|AIPerceptionComponent|GetActorsPerception (Variables|Default|GetAIPerception) _array_element))
          (for _array_element_2 (.LastSensedStimuli (Utilities|Struct|BreakActorPerceptionBlueprintInfo _info))
            (if (.bSuccessfullySensed (Utilities|Struct|BreakAIStimulus _array_element_2))
              (switch name (.Tag (Utilities|Struct|BreakAIStimulus _array_element_2))
                (:Default
                  (bind _asbp_player (Utilities|Casting|CastToBP_Player _array_element))
                  (AI|Components|Blackboard|SetValueasObject (AI|GetBlackboard 0) (Utilities|Name|MakeLiteralName "PlayerKey") _asbp_player)
                  (Variables|Default|SetIsFindPlayer true)
                  (CallFunction|PerceptionBreak))
                (:GrenadeNoise
                  (AI|Components|Blackboard|SetValueasVector (AI|GetBlackboard 0) (Utilities|Name|MakeLiteralName "NoiseLocationKey") (.StimulusLocation (Utilities|Struct|BreakAIStimulus _array_element_2)))
                  (bind _output_get (Variables|Default|SetHearingNoise true))
                  (AI|Components|Blackboard|SetValueasBool (AI|GetBlackboard 0) (Utilities|Name|MakeLiteralName "HearingNoiseKey") _output_get)
                  (Variables|Default|SetIsNoiseHearing true)
                  (CallFunction|PerceptionBreak))))))
        (:Completed
          ;[1 1 1] 못찾으면 Player 값을 Null 로
          (if (not (Variables|Default|GetIsFindPlayer))
            (AI|Components|Blackboard|SetValueasObject (AI|GetBlackboard 0) (Utilities|Name|MakeLiteralName "PlayerKey") 0)
            (if (not (Variables|Default|GetIsNoiseHearing))
              (bind _output_get_2 (Variables|Default|SetHearingNoise false))
              (AI|Components|Blackboard|SetValueasBool (AI|GetBlackboard 0) (Utilities|Name|MakeLiteralName "HearingNoiseKey") _output_get_2))))))))

(event Custom|PerceptionBreak
  (Utilities|Array|ForEachLoopwithBreak (Class|AIPerceptionComponent|GetCurrentlyPerceivedActors (Variables|Default|GetAIPerception))) ; enters at Break
)

(event EventBeginPlay)

(event EventTick
  (params (DeltaSeconds :type Float%20%28single-precision%29)))

(event EventPossess
  (params (PossessedPawn :type Pawn%20Object%20Reference))
  (bind _asbp_enemy_ai (Utilities|Casting|CastToBP_Enemy_AI PossessedPawn))
  (bind _output_get (Variables|Default|SetAIPawn _asbp_enemy_ai))
  (bind _behaviortree (Variables|/Game/Enemies/BP_Enemy_AI.BP_Enemy_AI_C|GetBehaviorTree _output_get)
    (:then
      (AI|RunBehaviorTree _behaviortree))
    (:else
      (Development|PrintString "행동 트리가 없음. AIController" true false))))

(fn ConstructionScript)