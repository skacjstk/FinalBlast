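; Ranged enemy Blueprint that fights with an assault rifle, hiding the inherited greatsword and setting a fire mode on BeginPlay.
; It spawns the rifle onto a holster socket, and attach, detach and equip events move it between hand and holster and update combat type.
; Aim info runs from just ahead of the enemy to the blackboard player's position, offset slightly against velocity.
; Aiming replication notifies the AnimInstance through an interface.
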(event EventBeginPlay
  (bind _assultrifle (Variables|Default|GetAssultRifle))
  (|CallParentFunction)
  (|AttachRifle)
  ;[1 1 1] 원거리캐는 GS 가리고 ,단발로
  (CallFunction|SetCurrentWeapon _assultrifle)
  (Rendering|SetActorHiddenInGame (Variables|Default|GetGreatSword) true)
  (Variables|/Game/Weapons/Ranged/BP_Ranged.BP_Ranged_C|SetcurrentWeaponFiremode _assultrifle "NewEnumerator5"))

(event Collision|EventActorBeginOverlap
  (params (OtherActor :type Actor%20Object%20Reference))
  (|CallParentFunction OtherActor) ; 지금 이 노드는 비활성 상태입니다. \n핀을 끌어서 다른 노드를 연결하면 활성화됩니다.
)

(event EventAttach
  (|CallParentFunction)
  (Transformation|AttachComponentToComponent (Variables|Default|GetAssultRifle) (Variables|Character|GetMesh) "Hand_Rifle" "KeepRelative" "KeepRelative" "KeepRelative" true)
  (Variables|Default|SetAttached true))

(event EventDetach
  (|CallParentFunction)
  (Transformation|AttachComponentToComponent (Variables|Default|GetAssultRifle) (Variables|Character|GetMesh) "Holster_Rifle" "KeepRelative" "KeepRelative" "KeepRelative" true)
  (Variables|Default|SetAttached false))

(event EventEquipped
  (|CallParentFunction)
  (CallFunction|SetCurrentWeapon (Variables|Default|GetAssultRifle))
  (Variables|Default|SetCombatType "NewEnumerator3"))

(event EventUnequipped
  (|CallParentFunction)
  (CallFunction|SetCurrentWeapon)
  (Variables|Default|SetCombatType "NewEnumerator0"))

(fn ConstructionScript
  (|CallParentFunction))

(fn WeaponAttach
  (Transformation|AttachComponentToComponent (Variables|Default|GetAssultRifle) (Variables|Character|GetMesh) "Hand_Rifle" "KeepRelative" "KeepRelative" "KeepRelative" true)
  (return true))

(fn OnRepIsAiming
  (bind _mesh (Variables|Character|GetMesh))
  (bind _returnvalue (Components|SkeletalMesh|GetAnimInstance _mesh))
  (if (Utilities|DoesObjectImplementInterface _returnvalue "/Game/Interfaces/IAnimInstance.IAnimInstance_C")
    (Class|IAnimInstance|IsAimingfromOwner(Message) _returnvalue (Variables|Default|GetIsAiming))))

(fn GetAimInfo
  (params (OutAimStart :type Vector%20%28by%20ref%29 :default "0, 0, 0") (OutAimEnd :type Vector%20%28by%20ref%29 :default "0, 0, 0") (OutAimDirection :type Vector%20%28by%20ref%29 :default "0, 0, 0"))
  (|SetBy-RefVar OutAimStart (+ (* (Transformation|GetActorForwardVector) 5e+01) (Transformation|GetActorLocation))) ; AimStart
  (Utilities|FlowControl|Sequence
    (:then_0
      (bind _asactor (Utilities|Casting|CastToActor (AI|Components|Blackboard|GetValueasObject (AI|GetBlackboard self) (Utilities|Name|MakeLiteralName "PlayerKey")))
        (:then
          (|SetBy-RefVar OutAimEnd (- (Transformation|GetActorLocation _asactor) (* (Transformation|GetVelocity _asactor) 0.07))) ; AimEnd
        )
        (:CastFailed
          (return false))))
    (:then_1
      (|SetBy-RefVar OutAimDirection (Math|Vector|GetUnitDirection(Vector) OutAimStart OutAimEnd)) ; AimDirection
      (return true))))