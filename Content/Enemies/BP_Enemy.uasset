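; BP_Enemy is a greatsword-wielding enemy character with a health bar, hidden from the player's minimap capture.
; Damage gets a BoneComponent multiplier, reduces StatusComponent health, reports to AI sense and shows floating text on the attacker.
; Hits flash the body through dynamic materials, and qualifying damage types trigger a stagger facing the attacker.
; Death ends player lock-on, launches a ragdoll, notifies the StageTrigger and destroys the actor after a delay.
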(event Custom|Die
  ;[1 1 1] 죽어가는 도중
  (bind _stagetrigger (Variables|Default|GetStageTrigger)
    (:then
      (Default|EnemyDie _stagetrigger))
    (:else
      (Development|PrintString "연계된게 없음" true false))))

(event Custom|Dead
  ;[1 1 1] 죽어가는 도중
  (Utilities|FlowControl|Sequence
    (:then_0
      (bind _asbp_player (Utilities|Casting|CastToBP_Player (Variables|Default|GetAttacker)))
      (Default|EndLockon _asbp_player))
    (:then_1
      (CallFunction|RagDoll)
      (CallFunction|Die)
      (Audio|PlaySoundatLocation "/Game/Sounds/Wave/Behavior/mixkit-quick-saber-cut-2158.mixkit-quick-saber-cut-2158" (Transformation|GetActorLocation) "0, 0, 0" 1.0 1.0 0.0 0 0 0)
      (Utilities|FlowControl|Delay 2.0)
      (Actor|DestroyActor))))

(event Custom|Attack
  (bind _currentweapon (Variables|Weapon|GetCurrentWeapon)
    (:then
      (Default|Attack _currentweapon))
    (:else)))

(event EventBeginPlay
  ;[1 1 1] 비긴플레이
  (Utilities|FlowControl|Sequence
    (:then_0
      (|AttachGreatSword))
    (:then_2
      (CallFunction|UpdateHealthBar))
    (:then_3
      (Utilities|FlowControl|Delay 0.2)
      (bind _asbp_player (Utilities|Casting|CastToBP_Player (Game|GetPlayerCharacter 0)))
      (Class|SceneCaptureComponent|HideActorComponents (Variables|/Game/Player/BP_Player.BP_Player_C|GetMinimapCapture _asbp_player) self false)
      (Class|SceneCaptureComponent|HideActorComponents (Variables|/Game/Player/BP_Player.BP_Player_C|GetMinimapCapture _asbp_player) (Variables|Weapon|GetGreatSword) false))
    (:then_4
      (CallFunction|SetCurrentWeapon (Variables|Weapon|GetGreatSword)))))

(event Game|Damage|EventAnyDamage
  (params (Damage :type Float%20%28single-precision%29) (DamageType :type Damage%20Type%20Object%20Reference) (InstigatedBy :type Controller%20Object%20Reference) (DamageCauser :type Actor%20Object%20Reference))
  ;[1 1 1] 피격 처리
  (if (Utilities|Enum|NotEqual(Enum) (Variables|Default|GetStateType) "NewEnumerator4")
    (Class|AISenseDamage|ReportDamageEvent self (Pawn|GetControlledPawn InstigatedBy) Damage (Transformation|GetActorLocation InstigatedBy))
    (|SetDamage Damage InstigatedBy DamageCauser)
    (bind _ishitreactiontype (Class|IDamageType|TriggerEffect(Message) DamageType (Variables|Default|GetDamageTypeEffectComponent) InstigatedBy))
    (if _ishitreactiontype
      (Variables|Default|SetStateType "NewEnumerator9") ; BT 파악용
      (Class|NavMovementComponent|StopMovementKeepPathing (Variables|Character|GetCharacterMovement))
      (Animation|PlayAnimMontage "/Game/Character/Montages/HitReaction_Montage.HitReaction_Montage" 1.5 "None")
      (|LookAtAttacker) ; 공격자 바라보게 하기
    )
    (|HitColor)
    (|CheckDead(FinishingBlow)) ; 마무리 일격 검사(죽음 검사)
  ))

(event EventDestroyed
  ;[1 1 1] 소멸자
  (Actor|DestroyActor (Variables|Weapon|GetGreatSword)))

(event Game|Damage|EventPointDamage
  (params (Damage :type Float%20%28single-precision%29) (DamageType :type Damage%20Type%20Object%20Reference) (HitLocation :type Vector :default "0, 0, 0") (HitNormal :type Vector :default "0, 0, 0") (HitComponent :type Primitive%20Component%20Object%20Reference) (BoneName :type Name :default "None") (ShotFromDirection :type Vector :default "0, 0, 0") (InstigatedBy :type Controller%20Object%20Reference) (DamageCauser :type Actor%20Object%20Reference) (HitInfo :type Hit%20Result%20Structure%20%28by%20ref%29))
  (bind _bonecomponent (Variables|Default|GetBoneComponent))
  (bind _asbp_ranged (Utilities|Casting|CastToBP_Ranged DamageCauser)
    (:then
      (bind _selectedmultiplepoint (Default|GetMultiplePoint _bonecomponent (.MultiplePoint (Utilities|Struct|BreakFGunData (Variables|/Game/Weapons/Ranged/BP_Ranged.BP_Ranged_C|GetWeaponData _asbp_ranged))) BoneName (Variables|Character|GetMesh)))
      (Variables|Default|SetMultipleDamage _selectedmultiplepoint))
    (:CastFailed
      (bind _1_0 (Default|GetSinglePoint _bonecomponent))
      (Variables|Default|SetMultipleDamage _1_0))))

(fn ConstructionScript
  (|SetDynamicMaterials_2)
  (CallFunction|SetBodyColor (Variables|BodyColor|GetBodyColor))
  (Rendering|Components|TextRender|SetText (Variables|Default|GetPawnName) (Utilities|Text|ToText(String) (Utilities|GetDisplayName self))))

(fn SetBodyColor
  (params (LBodyColor :type Linear%20Color%20Structure%20%28by%20ref%29))
  (for _array_element (Variables|Default|GetDynamicMaterials)
    (Rendering|Material|SetVectorParameterValue _array_element "BodyColor" LBodyColor :!class /Script/Engine.MaterialInstanceDynamic)))

(fn RagDoll
  (bind _mesh (Variables|Character|GetMesh))
  (Variables|/Script/Engine.SkeletalMeshComponent|SetGlobalAnimRateScale (Variables|Character|GetMesh) 0.0) ; 애니메이션 재생 중단
  (Collision|SetCollisionEnabled (Variables|Collision|GetCapsuleComponent) "NoCollision")
  (Physics|SetSimulatePhysics _mesh true)
  (Collision|SetCollisionEnabled _mesh "QueryAndPhysics")
  (Physics|AddForce _mesh (* (Math|Vector|GetUnitDirection(Vector) (Transformation|GetActorLocation (Variables|Default|GetAttacker)) (Transformation|GetActorLocation)) 5e+06) "None" false))

(fn LaunchActor
  (params (LaunchValue :type Float%20%28single-precision%29))
  (Transformation|AddActorWorldOffset (* (Class|KismetMathLibrary|VectorNormal2D (Transformation|GetActorForwardVector) 0.0001) LaunchValue)))

(fn UpdateHealthBar
  (bind _statuscomponent (Variables|Default|GetStatusComponent))
  (bind _aswb_stat (Utilities|Casting|CastToWB_Stat (UserInterface|GetUserWidgetObject (Variables|Default|GetHealthWidget))))
  (Default|UpdateStatBar _aswb_stat (Variables|/Game/Components/StatusComponent.StatusComponent_C|GetCurrentHealth _statuscomponent) (Variables|/Game/Components/StatusComponent.StatusComponent_C|GetMaxHealth _statuscomponent)))

(fn Attach)

(fn Detach)

(fn Equipped
  (Variables|Default|SetStateType "NewEnumerator0"))

(fn Unequipped
  (Variables|Default|SetStateType "NewEnumerator0"))

(fn Damaged
  (params (Damage :type Float%20%28single-precision%29) (DamageCauser :type Actor%20Object%20Reference))
  (Networking|SwitchHasAuthority
    (:Authority
      (Utilities|FlowControl|Sequence
        (:then_0
          (LocalVariables|SetAttacker'sFloatingDamageText (Actor|GetComponentbyClass DamageCauser "/Script/FinalBlast.FloatingDamageTextComponent")))
        (:then_1
          (bind _attacker_sfloatingdamagetext (LocalVariables|GetAttacker'sFloatingDamageText)
            (:then
              (Class|FloatingDamageTextComponent|AddFloatingTextCLIENT _attacker_sfloatingdamagetext (Utilities|Text|ToText(Float) Damage "HalfToEven" false true 1 324 0 0) (Transformation|GetActorLocation)))
            (:else)))))))

(fn GetAnimMontage
  (params (MontageKey :type Name :default "None"))
  (return 0 false))

(fn GetCombatType
  (return (Variables|Default|GetCombatType)))

(fn GetCurrentWeapon
  (return (Variables|Weapon|GetCurrentWeapon)))

(fn GetHealthBar
  (bind _aswb_stat (Utilities|Casting|CastToWB_Stat (UserInterface|GetUserWidgetObject (Variables|Default|GetHealthWidget))))
  (return _aswb_stat))

(fn GetOwnerParticleTrail
  (return 0))

(fn GetStaminaBar
  (return 0))

(fn GetStatusComponent
  (return 0))

(fn GetSubWeaponWidget
  (return 0))

(fn HitReactionEnd
  (bind _result (CallFunction|SetStateIdling))
  (return _result))

(fn IsStateAttacking
  (return (Utilities|Enum|Equal(Enum) (Variables|Default|GetStateType) "NewEnumerator3")))

(fn IsStateIdling
  (return (Utilities|Enum|Equal(Enum) (Variables|Default|GetStateType) "NewEnumerator0")))

(fn IsStateSpelling
  (return (Utilities|Enum|Equal(Enum) (Variables|Default|GetStateType) "NewEnumerator0")))

(fn RifleAttach
  (return false))

(fn RifleDetach
  (return false))

(fn RifleEquipped
  (return false))

(fn RifleUnEquipped
  (return false))

(fn SetCanMove
  (params (In :type Boolean))
  (return false))

(fn SetCurrentWeapon
  (params (NewWeapon :type BP%20Weapon%20Object%20Reference))
  (Utilities|IsValid (Variables|Weapon|GetCurrentWeapon)
    (:Is%20Valid
      (Default|OnUnEquipped (Variables|Weapon|GetCurrentWeapon)))
    (:Is%20Not%20Valid
      _))
  (Utilities|IsValid NewWeapon
    (:Is%20Valid
      (Default|OnEquipped NewWeapon)
      (bind _output_get (Variables|Weapon|SetCurrentWeapon NewWeapon))
      (return _output_get))
    (:Is%20Not%20Valid
      (Variables|Weapon|SetCurrentWeapon 0) ; Unarmed
      (return 0))))

(fn SetStateAttacking
  (Variables|Default|SetStateType "NewEnumerator3")
  (return false))

(fn SetStateIdling
  (Variables|Default|SetStateType "NewEnumerator0")
  (return false))

(fn SetStateSpelling
  (Variables|Default|SetStateType "NewEnumerator7")
  (return false))

(fn WeaponAttach
  (CallFunction|Attach)
  (return false))

(fn WeaponDetach
  (CallFunction|Detach)
  (return false))

(fn WeaponEquipped
  (CallFunction|Equipped)
  (return false))

(fn WeaponUnEquipped
  (CallFunction|Unequipped)
  (return false))