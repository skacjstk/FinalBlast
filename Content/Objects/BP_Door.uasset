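; BP_Door is a two-panel sliding door actor that opens and closes by player proximity when IsAutoOpen is set.
; Tick, enabled only in that mode, compares squared player distance to the squared threshold and toggles DoorState between closed and open.
; DoorOpen and DoorClose play or reverse the OpeningDoor timeline, whose curves drive SetDoorsLocation to rotate the lock and slide both panels in opposite directions.
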(event Custom|DoorClose
  (bind (_direction _doorlocation _lockrotation) (Timeline|OpeningDoor Reverse)
    (:Update
      (CallFunction|SetDoorsLocation _doorlocation _lockrotation))))

(event Custom|DoorOpen
  (bind (_direction _doorlocation _lockrotation) (Timeline|OpeningDoor Play)
    (:Update
      (CallFunction|SetDoorsLocation _doorlocation _lockrotation))))

(event EventBeginPlay
  (Actor|Tick|SetActorTickEnabled (Variables|Door|GetIsAutoOpen)))

(event Collision|EventActorBeginOverlap
  (params (OtherActor :type Actor%20Object%20Reference)))

(event EventTick
  (params (DeltaSeconds :type Float%20%28single-precision%29))
  (bind _needopentargetdistance (Variables|Default|GetNeedOpenTargetDistance))
  (bind _returnvalue (* _needopentargetdistance _needopentargetdistance))
  (switch int (Variables|Door|GetDoorState)
    (:0
      (bind _returnvalue_2 (CallFunction|GetDistancefromPlayerSquared))
      (if (<= _returnvalue_2 _returnvalue)
        (CallFunction|DoorOpen)
        (Variables|Door|SetDoorState 1)))
    (:1
      (bind _returnvalue_3 (CallFunction|GetDistancefromPlayerSquared))
      (if (> _returnvalue_3 _returnvalue)
        (CallFunction|DoorClose)
        (Variables|Door|SetDoorState 0)))))

(fn ConstructionScript)

(fn SetDoorsLocation
  (params (DoorLocation%28ratio%29 :type Float%20%28single-precision%29) (LockRotation%28ratio%29 :type Float%20%28single-precision%29))
  (bind _returnvalue (Math|Vector|MakeVector 0.0 2.5e+02 0.0))
  (bind _returnvalue_2 (Math|Vector|Lerp(Vector) "0, 0, 0" _returnvalue DoorLocation%28ratio%29))
  (Transformation|SetRelativeRotation (Variables|Default|GetLock) (Math|Rotator|MakeRotator (Math|Float|Lerp 0.0 (Math|Float|MakeLiteralFloat -9e+01) LockRotation%28ratio%29) 0.0 0.0) false false)
  (Transformation|SetRelativeLocation (Variables|Default|GetRightDoor) _returnvalue_2 false false)
  (Transformation|SetRelativeLocation (Variables|Default|GetLeftDoor) (* _returnvalue_2 -1.0) false false))

(fn GetDistancefromPlayerSquared
  (bind _returnvalue (Game|GetPlayerCharacter 0))
  (Utilities|IsValid _returnvalue
    (:Is%20Valid
      (return (Class|KismetMathLibrary|VectorDistanceSquared (Transformation|GetActorLocation) (Transformation|GetActorLocation _returnvalue))))))