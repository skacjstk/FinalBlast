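; BP_TargetPoint is a checkpoint-style target actor with a box trigger and a circle plane marker, driven by a BP_TargetPointManager passed in through SetPointManager.
; AppearPoint and DisAppearPoint toggle the marker's visibility and the box's query collision together.
; Any overlap, given a valid manager, calls NextPointEnable, disables collision and turns the marker green.
; The construction script sizes the box, places the marker at its bottom and creates the dynamic material.
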(event Custom|OnCollision
  ;[1 1 1] 충돌체 끄거나 켜기
  (Collision|SetCollisionEnabled (Variables|Default|GetBox) "QueryOnly"))

(event Custom|OffCollision
  ;[1 1 1] 충돌체 끄거나 켜기
  (Collision|SetCollisionEnabled (Variables|Default|GetBox) "NoCollision"))

(event Custom|SetPointManager
  (params (NewParam :type Actor%20Object%20Reference))
  (bind _asbp_target_point_manager (Utilities|Casting|CastToBP_TargetPointManager NewParam)
    (:then
      (Variables|Default|SetPointManager _asbp_target_point_manager))
    (:CastFailed
      (Development|PrintString "경고: PointManager 할당 실패" true false))))

(event Custom|AppearPoint
  (CallFunction|OnCollision)
  (Development|SetHiddeninGame (Variables|Default|GetPlaneCircle) false false))

(event Custom|DisAppearPoint
  (CallFunction|OffCollision)
  (Development|SetHiddeninGame (Variables|Default|GetPlaneCircle) true false))

(event Collision|EventActorBeginOverlap
  (params (OtherActor :type Actor%20Object%20Reference))
  ;[1 1 1] 충돌시 초록색으로 변경 및 매니저에게 이벤트 호출
  (bind _pointmanager (Variables|Default|GetPointManager)
    (:then
      (Default|NextPointEnable _pointmanager)
      (CallFunction|OffCollision)
      (Rendering|Material|SetVectorParameterValue (Variables|Default|GetMatDynamic) "Color" "(R=0.000000,G=1.000000,B=0.000000,A=1.000000)" :!class /Script/Engine.MaterialInstanceDynamic))
    (:else)))

(fn ConstructionScript
  (bind _collisionsize (Variables|Default|GetCollisionSize))
  (bind _planecircle (Variables|Default|GetPlaneCircle))
  (Components|Box|SetBoxExtent (Variables|Default|GetBox) _collisionsize true)
  (Transformation|SetRelativeLocation (Variables|Default|GetPlaneCircle) (Math|Vector|MakeVector 0.0 0.0 (* (.Z (Math|Vector|BreakVector _collisionsize)) -1.0)) false false)
  (bind _returnvalue (Rendering|Material|CreateDynamicMaterialInstance _planecircle 0 (Rendering|Material|GetMaterial _planecircle 0) "None" :!class /Script/Engine.PrimitiveComponent))
  (Variables|Default|SetMatDynamic _returnvalue))