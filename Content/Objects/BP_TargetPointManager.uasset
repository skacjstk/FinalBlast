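; BP_TargetPointManager runs an ordered sequence of target points in a stage, showing only the first at BeginPlay.
; Each NextPointEnable call advances the index, reveals the next point, plays a shutter sound and spawns an arrow.
; The BP_Arrow sits midway between previous and current points, lowered by box extent, aimed along the path and stretched by distance.
; Once the index reaches the point count, it calls StageClear on a valid StageTrigger.
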(event Custom|NextPointEnable
  (bind _result (Math|Integer|IncrementInt (Variables|Default|GetcurrentPoint))
    (:%20%20
      (Math|Integer|CompareInt _result (Variables|Default|GetMaxPointCount)
        (:>
          (bind _stagetrigger (Variables|Default|GetStageTrigger :!label _label)
            (:then
              (Default|StageClear _stagetrigger))
            (:else)))
        (:==
          (goto _label))
        (:<
          (Default|AppearPoint (Utilities|Array|Get(acopy) (Variables|Default|GetTargetPoints) _result))
          (Audio|PlaySound2D "/Engine/VREditor/Sounds/UI/Camera_Shutter.Camera_Shutter" 1.0 1.0 0.0 0 0)
          (CallFunction|SpawnArrow))))))

(event Custom|SpawnArrow
  (bind _targetpoints (Variables|Default|GetTargetPoints))
  (bind _currentpoint (Variables|Default|GetcurrentPoint))
  (bind _returnvalue (- _currentpoint 1))
  (bind _output (Utilities|Array|Get(acopy) _targetpoints _currentpoint))
  (bind _returnvalue_2 (Transformation|GetActorLocation _output))
  (bind _returnvalue_3 (Math|Integer|Max(Integer) _returnvalue))
  (bind _output_2 (Utilities|Array|Get(acopy) _targetpoints _returnvalue_3))
  (bind _returnvalue_4 (Transformation|GetActorLocation _output_2))
  (Game|SpawnActorfromClass "/Game/Objects/BP_Arrow.BP_Arrow_C" (Math|Transform|MakeTransform (- (Math|Vector|Lerp(Vector) _returnvalue_2 _returnvalue_4 0.5) (Math|Vector|MakeVector 0.0 0.0 (.z (Components|Box|GetScaledBoxExtent (Variables|/Game/Objects/BP_TargetPoint.BP_TargetPoint_C|GetBox _output))))) (Math|Conversions|RotationFromXVector (Math|Vector|GetUnitDirection(Vector) _returnvalue_4 _returnvalue_2)) (Math|Vector|MakeVector 1.0 (Math|Float|Max(Float) (/ (Transformation|GetDistanceTo _output _output_2) 1.5e+02) 1.0) 1.0)) "Undefined" 0 0))

(event EventBeginPlay
  (bind _targetpoints (Variables|Default|GetTargetPoints))
  ;[1 1 1] 소유한 TargetPoints 에게 주인 세팅 및 첫번째 TargetPoint 제외 가리기
  (for _array_element _targetpoints
    (Default|SetPointManager _array_element self)
    (Default|DisAppearPoint _array_element))
  (Default|AppearPoint (Utilities|Array|Get(acopy) _targetpoints)))

(fn ConstructionScript
  (Variables|Default|SetMaxPointCount (Utilities|Array|Length (Variables|Default|GetTargetPoints))))