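; BP_Move is an actor that moves itself continuously along its local Y axis while rotating.
; Each Tick applies a fixed local rotation step, then a delta-time-scaled local offset, both without sweep, so the offset follows the changing orientation.
; The rotation step is not scaled by delta time, so the path depends on frame rate.
; Disconnected nodes hold a combined-transform move and debug prints of the Sphere's relative and world location.
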(event EventBeginPlay)

(event Collision|EventActorBeginOverlap
  (params (OtherActor :type Actor%20Object%20Reference)))

(event EventTick
  (params (DeltaSeconds :type Float%20%28single-precision%29))
  (bind _returnvalue (* DeltaSeconds 4e+02))
  (bind _returnvalue_2 (Math|Vector|MakeVector 0.0 _returnvalue 0.0))
  (bind _returnvalue_3 (Math|Transform|MakeTransform _returnvalue_2 "0.000000,1.000000, 0"))
  (Transformation|AddActorLocalRotation (.rotation _returnvalue_3) false false)
  (Transformation|AddActorLocalOffset (.location _returnvalue_3) false false))

(fn ConstructionScript)