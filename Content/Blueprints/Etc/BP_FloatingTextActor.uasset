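; BP_FloatingTextActor is an actor that shows one piece of floating text, such as damage text, through a WB_FloatingDamageText widget component.
; Its Initalize event only stores the text, which BeginPlay passes to the widget, so the value must be set before BeginPlay runs.
; BeginPlay also binds to the widget's animation-finished event, and HandleAnimFinished destroys the actor when the animation ends.
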(event EventBeginPlay
  (bind _aswb_floating_damage_text (Utilities|Casting|CastToWB_FloatingDamageText (UserInterface|GetUserWidgetObject (Variables|Default|GetWidget))))
  (EventDispatchers|BindEventtoAnimFinished _aswb_floating_damage_text (EventDispatchers|CreateEvent :!event HandleAnimFinished))
  (Default|Initialize _aswb_floating_damage_text (Variables|Default|GetText)))

(event EventInitalize
  (params (text :type Text%20%28by%20ref%29))
  (Variables|Default|SetText text))

(fn ConstructionScript)

(fn HandleAnimFinished
  ;[1 1 1] 애니메이션 끝날때 액터 삭제
  (Actor|DestroyActor))