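; BP_DamageText is a self-destroying floating text actor that shows a damage value set through SetDamageText.
; On BeginPlay, a timeline's vector track drives the text's height offset from the spawn location (X) and the actor's uniform scale (Y).
; Each update also copies player 0's control roll and pitch to the text with yaw fixed at 180, then the actor is destroyed when the timeline finishes.
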(event EventBeginPlay
  (bind _returnvalue (Game|GetPlayerController 0))
  (bind _textrender (Variables|Default|GetTextRender))
  (bind _returnvalue_2 (Pawn|GetControlRotation _returnvalue :!class /Script/Engine.Controller))
  (Variables|Default|SetStartLocation (Transformation|GetActorLocation))
  (bind _result (Timeline|Timeline Play)
    (:Update
      (Transformation|SetWorldLocation _textrender (+ (Variables|Default|GetStartLocation) (Math|Vector|MakeVector 0.0 0.0 (.X (Math|Vector|BreakVector _result)))) false false)
      (Transformation|SetWorldRotation _textrender (Math|Rotator|MakeRotator (.roll _returnvalue_2) (.pitch _returnvalue_2) 1.8e+02) false false)
      (Transformation|SetActorScale3D (Math|Conversions|ToVector(Float) (.Y (Math|Vector|BreakVector _result)))))
    (:Finished
      (Actor|DestroyActor))))

(fn ConstructionScript)

(fn SetDamageText
  (params (Damage :type Float%20%28single-precision%29))
  (Rendering|Components|TextRender|SetText (Variables|Default|GetTextRender) (Utilities|Text|ToText(Float) Damage "HalfToEven")))