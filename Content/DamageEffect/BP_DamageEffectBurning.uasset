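; BP_DamageEffectBurning is a damage effect actor that burns the actor it is attached to over time.
; On BeginPlay it runs the parent setup, then sets its life span slightly past InitialLifeSpan so it cleans itself up.
; A looping one-second timer applies fixed damage to the attach parent, crediting the instigator's controller.
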(event Custom|TargetBurning
  (Game|Damage|ApplyDamage (Actor|GetAttachParentActor) 5.0 (Game|GetInstigatorController) 0))

(event EventBeginPlay
  (|CallParentFunction)
  (Actor|SetLifeSpan (+ (Variables|Default|GetInitialLifeSpan) 0.1))
  (Utilities|Time|SetTimerbyEvent (delegate Custom|TargetBurning) 1.0 true))

(event Collision|EventActorBeginOverlap
  (params (OtherActor :type Actor%20Object%20Reference))
  (|CallParentFunction OtherActor) ; 지금 이 노드는 비활성 상태입니다. \n핀을 끌어서 다른 노드를 연결하면 활성화됩니다.
)

(event EventTick
  (params (DeltaSeconds :type Float%20%28single-precision%29))
  (|CallParentFunction DeltaSeconds) ; 지금 이 노드는 비활성 상태입니다. \n핀을 끌어서 다른 노드를 연결하면 활성화됩니다.
)

(fn ConstructionScript
  (|CallParentFunction))