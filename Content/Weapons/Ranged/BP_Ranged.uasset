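; Base ranged weapon that loads gun, ammo and ballistics data tables and handles aiming, firing and reloading.
; A paused looping timer paces shots by RPM and fire mode; each shot line-traces, re-tracing past one-way shields, then applies enemy-only damage or decals.
; Empty fire triggers a reload montage, with Reloaded refilling the magazine from reserves.
; OnRep functions report ammo, fire mode and aim state; melee combo functions also remain.
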(event Custom|DamageEffect)

(event Custom|FireTickTimer
  ;[1 1 1] Fire에서 UnPause로 실행
  (bind _output_get (Variables|Fire|SetRemainSingleFireDelay (- (Variables|Fire|GetRemainSingleFireDelay) (Math|Float|MakeLiteralFloat 0.016667))))
  (if (<= _output_get 0.0)
    (if (and (Utilities|Select :Index (Variables|Data|GetcurrentWeaponFiremode) :NewEnumerator1 (Variables|Default|GetIsFiring) :NewEnumerator2 (> (Variables|Data|GetNumOfOneClickShot) 0) :NewEnumerator5 (> (Variables|Data|GetNumOfOneClickShot) 0) :NewEnumerator6 false) (Variables|Default|GetCanFire))
      (CallFunction|TryFire) ; 잔탄 검사는 여기에 있음
      (Variables|Fire|SetRemainSingleFireDelay (Variables|Fire|GetMaxSingleFireDelay))
      (else
        (Utilities|Time|PauseTimerbyHandle (Variables|Fire|GetFireTickTimerHandle))
        (Variables|Data|SetNumOfOneClickShot (CallFunction|GetMaxOneClickShot))
        (CallFunction|ReleaseAttack)))))

(event Custom|Reload
  (bind _returnvalue (Components|GetOwner))
  ;[1 1 1] 재장전( 노티파이에서 재생해서 다시 Reloaded 함수를 호출하는 구조 )
  (if (and (not (Variables|Default|GetIsReloading)) (Utilities|DoesObjectImplementInterface _returnvalue "/Game/Interfaces/IState.IState_C"))
    (if (> (Variables|Data|GetMaxAmmo) 0)
      (bind (_animmontage _findsuccess) (Class|IState|GetAnimMontage(Message) _returnvalue "Reload"))
      (if _findsuccess
        (Class|IState|PlayAnimMontageOwner(Message) _returnvalue _animmontage)
        (Variables|Default|SetIsReloading true)))))

(event Custom|FireFail
  (CallFunction|Reload))

(event Custom|ResetVariableEvent
  (Variables|Default|SetIsReloading false)
  (Variables|Default|SetCanFire true))

(event Custom|ZoomIn
  ;[1 1 1] Zoom 이벤트
  (bind _asbp_player (Utilities|Casting|CastToBP_Player (Components|GetOwner)))
  (Variables|Default|SetOwnerPlayer _asbp_player)
  (bind _fov (Timeline|Timeline_FOV Play)
    (:Update
      (Camera|SetFieldOfView (Variables|/Game/Player/BP_Player.BP_Player_C|GetCamera (Variables|Default|GetOwnerPlayer)) _fov))))

(event Custom|ZoomOut
  ;[1 1 1] Zoom 이벤트
  (bind _asbp_player (Utilities|Casting|CastToBP_Player (Components|GetOwner)))
  (Variables|Default|SetOwnerPlayer _asbp_player)
  (bind _fov (Timeline|Timeline_FOV Reverse)
    (:Update
      (Camera|SetFieldOfView (Variables|/Game/Player/BP_Player.BP_Player_C|GetCamera (Variables|Default|GetOwnerPlayer)) _fov))))

(event EventBeginPlay
  (bind _weapondata (Variables|Data|GetWeaponData))
  ;[1 1 1] 비긴플레이: 데이터테이블(콤보 몽타쥬) 읽어오기
  (|CallParentFunction)
  (Utilities|FlowControl|Sequence
    (:then_0
      (|ReadGunData))
    (:then_1
      (|ReadAmmoData) ; 여기에 장탄 수 있음
    )
    (:then_2
      (|ReadBallisticsData))
    (:then_3
      (bind _output_get (Variables|Fire|SetMaxSingleFireDelay (/ 6e+01 (Math|Conversions|ToFloat(Integer) (.rpm _weapondata)))))
      (Variables|Fire|SetRemainSingleFireDelay _output_get)
      (Variables|Data|SetcurrentWeaponFiremode (.firemodetype _weapondata)))
    (:then_4
      (bind _returnvalue (Utilities|Time|SetTimerbyEvent (delegate Custom|FireTickTimer) (Math|Float|MakeLiteralFloat 0.016667) true))
      (bind _output_get_2 (Variables|Fire|SetFireTickTimerHandle _returnvalue))
      (Utilities|Time|PauseTimerbyHandle _output_get_2))
    (:then_5
      (EventDispatchers|BindEventtoFailFire (EventDispatchers|CreateEvent :!event Custom|FireFail)))
    (:then_6
      (EventDispatchers|BindEventtoResetVariable (EventDispatchers|CreateEvent :!event Custom|ResetVariableEvent)))))

(fn ConstructionScript
  (|CallParentFunction))

(fn Attack
  (|CallParentFunction)
  (CallFunction|OnAim)
  (Variables|Default|SetIsFiring true)
  (Utilities|Time|UnpauseTimerbyHandle (Variables|Fire|GetFireTickTimerHandle)))

(fn PlayComboMontage
  (bind _melee_datas (Variables|Combo|GetMelee%20Datas))
  (bind _combocount (Variables|Combo|GetComboCount))
  (bind _output (Utilities|Array|Get(acopy) _melee_datas _combocount))
  (bind _ascharacter (Utilities|Casting|CastToCharacter (Components|GetOwner)))
  (if (> (Utilities|Array|Length _melee_datas) _combocount)
    (Animation|PlayAnimMontage _ascharacter (.montage _output) (.playrate _output) (.startsection _output))
    (CallFunction|SetCanMove (.canmove _output))
    (Variables|Default|SetIsSmashing false)))

(fn PlayNextCombo
  (if (Variables|Combo|GetSucceedCombo)
    (if (Variables|Combo|GetSucceedSmash)
      (CallFunction|PlaySmashMontage)
      (Math|Integer|IncrementInt (Variables|Combo|GetSamshCount)
        (:%20%20
          _))
      (else
        (Math|Integer|IncrementInt (Variables|Combo|GetComboCount)
          (:%20%20
            (CallFunction|PlayComboMontage)))))
    (Variables|Combo|SetSucceedCombo false)
    (Variables|Combo|SetSucceedSmash false)
    (Variables|Default|SetIsLastCombo (== (- (Utilities|Array|Length (Variables|Combo|GetMelee%20Datas)) 1) (Variables|Combo|GetComboCount)))))

(fn OnCollision
  (params (FistCollisionType :type EFistCollisionType%20Enum :default "NewEnumerator0") (SmashHitIndex :type Integer))
  (Variables|Combo|SetSmashHitIndex SmashHitIndex))

(fn OffCollision
  (Utilities|Array|Clear (Variables|Default|GetHittedActors)))

(fn SendDamage
  (params (Other%20Actor :type Actor%20Object%20Reference) (Damage :type Float%20%28single-precision%29) (hitResult :type Hit%20Result%20Structure%20%28by%20ref%29) (DamageTypeClass :type Damage%20Type%20Class%20Reference) (Event%20Instigator :type Controller%20Object%20Reference))
  (bind _myteamid (Class|IState|GetMyTeamID(Message) (Components|GetOwner)))
  (bind _isenemy (Class|IState|IsEnemy(Message) Other%20Actor _myteamid))
  (if _isenemy
    (bind _result (|CallParentFunction Other%20Actor Damage hitResult DamageTypeClass Event%20Instigator))
    (if _result
      (return true))))

(fn EndAttack
  ;[1 1 1] 공격 끝
  (|CallParentFunction)
  (CallFunction|SetStateIdling)
  (Variables|Combo|SetComboCount 0)
  (Variables|Combo|SetSamshCount 0)
  (CallFunction|SetCanMove true)
  (Variables|Combo|SetSucceedCombo false)
  (Variables|Default|SetIsLastCombo false)
  (Variables|Combo|SetSucceedSmash false)
  (CallFunction|EndCombo))

(fn StartCombo)

(fn EndCombo)

(fn PlaySmashMontage
  (bind (_statuscomp _isvalid) (CallFunction|GetOwnertoStatusComponent))
  (bind (_statuscomp_2 _isvalid_2) (CallFunction|GetOwnertoStatusComponent))
  (bind _samshcount (Variables|Combo|GetSamshCount))
  (bind _combocount (Variables|Combo|GetComboCount))
  (bind _smashdatas (Variables|Combo|GetSmashDatas))
  (bind _returnvalue (Utilities|String|ToString(Integer) _samshcount))
  (bind _returnvalue_2 (Utilities|String|ToString(Integer) _combocount))
  (bind _returnvalue_3 (Utilities|String|Append _returnvalue_2 "_" _returnvalue))
  (bind _returnvalue_4 (Utilities|String|StringToName _returnvalue_3))
  (bind _value (Utilities|Map|Find _smashdatas _returnvalue_4))
  (bind _ascharacter (Utilities|Casting|CastToCharacter (Components|GetOwner)))
  (if _isvalid
    ;[1 1 1] 스테이터스 Get 구현을 한 개체만 검사 (Enemy는 구현을 안했어)
    (if (>= (Variables|/Game/Components/StatusComponent.StatusComponent_C|GetCurrentStamina _statuscomp) (.needstaminaamount _value))
      (Animation|PlayAnimMontage _ascharacter (.montage _value) (.playrate _value) (.startsection _value) :!label _label)
      (CallFunction|SetCanMove (.canmove _value))
      (Variables|Default|SetIsSmashing true)
      ;[1 1 1] 플레이어만 스태미나 감소
      (if _isvalid_2
        (Default|DecreaseStamina _statuscomp_2 (.needstaminaamount _value))))
    (else
      (goto _label))))

(fn Smash
  (|CallParentFunction)
  (CallFunction|OnAim))

(fn CanAttack
  (return true))

(fn OnAim
  (bind _returnvalue (Components|GetOwner))
  (if (not (Variables|Default|GetIsAiming))
    (Utilities|FlowControl|Sequence
      (:then_0
        (bind _ascharacter (Utilities|Casting|CastToCharacter _returnvalue))
        (Variables|/Script/Engine.Pawn|SetbUseControllerRotationYaw _ascharacter true)
        (Variables|/Script/Engine.CharacterMovementComponent|SetbOrientRotationToMovement (Variables|/Script/Engine.Character|GetCharacterMovement _ascharacter) false)
        (Variables|Default|SetIsAiming true)
        (Variables|/Script/Engine.CharacterMovementComponent|SetMaxWalkSpeed (Variables|/Script/Engine.Character|GetCharacterMovement _ascharacter) 4e+02))
      (:then_1
        (bind _asbp_player (Utilities|Casting|CastToBP_Player _returnvalue))
        (Variables|/Script/Engine.SpringArmComponent|SetbEnableCameraLag (Variables|/Game/Player/BP_Player.BP_Player_C|GetSpringArm _asbp_player) false)
        (Variables|/Script/Engine.SpringArmComponent|SetbEnableCameraRotationLag (Variables|/Game/Player/BP_Player.BP_Player_C|GetSpringArm _asbp_player) false)
        (Variables|/Script/Engine.SpringArmComponent|SetTargetArmLength (Variables|/Game/Player/BP_Player.BP_Player_C|GetSpringArm _asbp_player) 1e+02)
        (Variables|/Script/Engine.SpringArmComponent|SetSocketOffset (Variables|/Game/Player/BP_Player.BP_Player_C|GetSpringArm _asbp_player) "0,60.000000,5.000000")
        (CallFunction|Zoomin)))))

(fn OffAim
  (bind _returnvalue (Components|GetOwner))
  (if (Variables|Default|GetIsAiming)
    (Utilities|FlowControl|Sequence
      (:then_0
        (bind _ascharacter (Utilities|Casting|CastToCharacter _returnvalue))
        (Variables|/Script/Engine.Pawn|SetbUseControllerRotationYaw _ascharacter false)
        (Variables|/Script/Engine.CharacterMovementComponent|SetbOrientRotationToMovement (Variables|/Script/Engine.Character|GetCharacterMovement _ascharacter) true)
        (Variables|Default|SetIsAiming false)
        (Variables|/Script/Engine.CharacterMovementComponent|SetMaxWalkSpeed (Variables|/Script/Engine.Character|GetCharacterMovement _ascharacter) 6e+02))
      (:then_1
        (bind _asbp_player (Utilities|Casting|CastToBP_Player _returnvalue))
        (Variables|/Script/Engine.SpringArmComponent|SetSocketOffset (Variables|/Game/Player/BP_Player.BP_Player_C|GetSpringArm _asbp_player) "0, 0, 0")
        (Variables|/Script/Engine.SpringArmComponent|SetTargetArmLength (Variables|/Game/Player/BP_Player.BP_Player_C|GetSpringArm _asbp_player) 3e+02)
        (Variables|/Script/Engine.SpringArmComponent|SetbEnableCameraLag (Variables|/Game/Player/BP_Player.BP_Player_C|GetSpringArm _asbp_player) true)
        (Variables|/Script/Engine.SpringArmComponent|SetbEnableCameraRotationLag (Variables|/Game/Player/BP_Player.BP_Player_C|GetSpringArm _asbp_player) true)
        (CallFunction|ZoomOut)))))

(fn OnRepIsAiming
  (bind _ascharacter (Utilities|Casting|CastToCharacter (Components|GetOwner)))
  (if (Utilities|DoesObjectImplementInterface (Components|SkeletalMesh|GetAnimInstance (Variables|/Script/Engine.Character|GetMesh _ascharacter)) "/Game/Interfaces/IAnimInstance.IAnimInstance_C")
    (Class|IAnimInstance|IsAimingfromOwner(Message) (Components|SkeletalMesh|GetAnimInstance (Variables|/Script/Engine.Character|GetMesh _ascharacter)) (Variables|Default|GetIsAiming))))

(fn ReleaseRightClick
  (|CallParentFunction)
  (CallFunction|OffAim))

(fn TryFire
  (Utilities|FlowControl|Sequence
    (:then_0
      ;[1 1 1] 발사 검사 및 발사 성공시 아래 시퀀스 진행
      (Variables|Default|SetCanFire (> (Variables|Data|GetCurrentAmmo) 0)))
    (:then_1
      (if (Variables|Default|GetCanFire)
        (|Fire)
        (else
          (Default|CallFailFire))))))

(fn ReleaseAttack
  (|CallParentFunction)
  (Variables|Default|SetIsFiring false))

(fn OnRepCurrentWeaponFiremode
  (switch Utilities|FlowControl|Switch|SwitchonEFiremodeType (Variables|Data|GetcurrentWeaponFiremode)
    (:NewEnumerator1
      (Variables|Data|SetNumOfOneClickShot 5))
    (:NewEnumerator2
      (Variables|Data|SetNumOfOneClickShot 3))
    (:NewEnumerator5
      (Variables|Data|SetNumOfOneClickShot 1)))
  (Class|IWeapon|ChangeCurrentFiremode(Message) (Components|GetOwner) (Variables|Data|GetcurrentWeaponFiremode)))

(fn GetMaxOneClickShot
  (return (Utilities|Select :Index (Variables|Data|GetcurrentWeaponFiremode) :NewEnumerator1 5 :NewEnumerator2 3 :NewEnumerator5 1 :NewEnumerator6 0)))

(fn Reloaded
  (bind _baseammodata (Variables|Data|GetBaseAmmoData))
  (bind _magazine (Utilities|Struct|BreakFAmmoData _baseammodata))
  (|CallParentFunction)
  (Variables|Default|SetCanFire true)
  (Variables|Default|SetIsReloading false)
  (Variables|Data|SetMaxAmmo (+ (Variables|Data|GetCurrentAmmo) (Variables|Data|GetMaxAmmo)))
  (if (>= (Variables|Data|GetMaxAmmo) _magazine)
    (Variables|Data|SetCurrentAmmo _magazine)
    (Variables|Data|SetMaxAmmo (- (Variables|Data|GetMaxAmmo) _magazine))
    (else
      (Variables|Data|SetCurrentAmmo (Variables|Data|GetMaxAmmo))
      (Variables|Data|SetMaxAmmo 0))))

(fn OnRepCurrentAmmo
  (Class|IWeapon|ChangeCurrentAmmo(Message) (Components|GetOwner) (Variables|Data|GetCurrentAmmo)))

(fn OnRepMaxAmmo
  (Class|IWeapon|ChangeMaxAmmo(Message) (Components|GetOwner) (Variables|Data|GetMaxAmmo)))

(fn SwitchFiremode
  (|CallParentFunction)
  (Variables|Data|SetcurrentWeaponFiremode (Utilities|Enum|ByteToEnumEFiremodeType (Class|KismetMathLibrary|PercentByteByte (+ (Variables|Data|GetcurrentWeaponFiremode) 1) (LocalVariables|GetMax)))))

(fn ChangeCurrentAmmo
  (params (ChangeAmmo :type Integer%20%28by%20ref%29))
  (return false))

(fn ChangeCurrentFiremode
  (params (NewParam :type EFiremodeType%20Enum :default "NewEnumerator1"))
  (return false))

(fn ChangeMaxAmmo
  (params (Change :type Integer%20%28by%20ref%29))
  (return false))

(fn GetCombatType
  (return (Variables|Default|GetCombatType)))

(fn GetCurrentWeapon
  (return 0))

(fn GetOwnerParticleTrail
  (return 0))

(fn GetSubWeaponWidget
  (return 0))

(fn RifleAttach
  (return false))

(fn RifleDetach
  (return false))

(fn RifleEquipped
  (return false))

(fn RifleUnEquipped
  (return false))

(fn SetCurrentWeapon
  (params (NewWeapon :type BP%20Weapon%20Object%20Reference))
  (return 0))

(fn WeaponAttach
  (return false))

(fn WeaponDetach
  (return false))

(fn WeaponEquipped
  (return false))

(fn WeaponUnEquipped
  (return false))