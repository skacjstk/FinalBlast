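; BP_Projectile is a ranged-weapon projectile that destroys itself when its static mesh begins overlapping another actor, ignoring its owner's owner.
; For a BP_OneWayShield, it first calls IsPathableWall with itself and its collision mesh.
; Both results of that check end in the same owner test and destroy, so the returned value does not change whether the projectile is destroyed.
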(event OnComponentBeginOverlap(StaticMesh)
  (params (OverlappedComponent :type Primitive%20Component%20Object%20Reference) (OtherActor :type Actor%20Object%20Reference) (OtherComp :type Primitive%20Component%20Object%20Reference) (OtherBodyIndex :type Integer) (bFromSweep :type Boolean) (SweepResult :type Hit%20Result%20Structure%20%28by%20ref%29))
  (bind _returnvalue (Components|GetOwner))
  (bind _returnvalue_2 (Components|GetOwner _returnvalue))
  (bind _returnvalue_3 (!= OtherActor _returnvalue_2))
  (bind _asbp_one_way_shield (Utilities|Casting|CastToBP_OneWayShield OtherActor)
    (:then
      (bind _cannotpath (Default|IsPathableWall _asbp_one_way_shield self (Variables|Default|GetStaticMesh)))
      (if (and _cannotpath _returnvalue_3)
        (Actor|DestroyActor :!label _label)
        (else
          (if _returnvalue_3 :!label _label_2
            (goto _label)))))
    (:CastFailed
      (goto _label_2))))

(event EventBeginPlay)

(event Collision|EventActorBeginOverlap
  (params (OtherActor :type Actor%20Object%20Reference)))

(event EventTick
  (params (DeltaSeconds :type Float%20%28single-precision%29)))

(fn ConstructionScript)