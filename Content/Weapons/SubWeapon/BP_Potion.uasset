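; BP_Potion is a sub-weapon item that heals the owning character when used.
; On StartSubweapon, it checks whether use is allowed, then raises health through the owner's StatusComponent and plays a sound at the character's location.
; It then registers the use, initializes the SubWeaponComponent for the selected container slot, and refreshes the regen timer from the item's cooldown and use-limit properties.
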(event EventBeginPlay
  (|CallParentFunction) ; 지금 이 노드는 비활성 상태입니다. \n핀을 끌어서 다른 노드를 연결하면 활성화됩니다.
)

(event EventStartSubweapon
  (params (SelectedItemIndex :type Integer))
  (bind _iswproperty (Variables|Default|GetISWProperty))
  (bind _subweaponcomponent (Variables|Default|GetSubWeaponComponent))
  (bind (_itemname _hascooltime _hasuselimit _cooltime _inituselimit) (Utilities|Struct|BreakFISWProperty _iswproperty))
  (bind _canuse (CallFunction|CheckCanUseSubWeapon _iswproperty))
  (if _canuse
    (Default|IncreaseHealth (Actor|GetComponentbyClass (CallFunction|GetOwnertoCharacter) "/Game/Components/StatusComponent.StatusComponent_C") (Variables|Default|GetHealAmount))
    (Audio|PlaySoundatLocation "/Game/Sounds/Wave/Behavior/FairyDrop.FairyDrop" (Transformation|GetActorLocation (CallFunction|GetOwnertoCharacter)) "0, 0, 0" 1.0 1.0 0.0 0 0 0)
    (CallFunction|UseSubWeapon _iswproperty)
    (Default|InitMemberValue _subweaponcomponent SelectedItemIndex -1 false)
    (Default|RefreshRegenTimer _subweaponcomponent _cooltime _hasuselimit _inituselimit)))

(fn ConstructionScript
  (|CallParentFunction))