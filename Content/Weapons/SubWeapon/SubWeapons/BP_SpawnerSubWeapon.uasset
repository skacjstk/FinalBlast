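; BP_SpawnerSubWeapon is a sub-weapon that spawns the selected item actor, such as a black hole or shield, in front of its owning character.
; StartSubweapon spawns the current SubWeaponItems entry with the spawner as owner.
; GetSpawnFrontVector offsets from the Spine_03 socket, using control yaw alone or full control rotation per the item's IsViewFront flag.
; SetSubWeaponIcon fills container-widget slots with item icons and returns the item count.
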(event EventBeginPlay
  ;[1 1 1] 스포너가 가진 아이템 갯수 저장
  (|CallParentFunction)
  (Variables|Default|SetInitialContainerIndex (Utilities|Array|Length (Variables|Default|GetSubWeaponItems))))

(event EventStartSubweapon
  (bind _subweaponitems (Variables|Default|GetSubWeaponItems))
  (bind _currentitem (Variables|Default|GetcurrentItem))
  (bind _output (Utilities|Array|Get(acopy) _subweaponitems _currentitem))
  ;[1 1 1] 여기서 블랙홀, 실드 생성 혹은 삭제
  (Game|SpawnActorfromClass (.subweapontype _output) (CallFunction|GetSpawnFrontVector (.isviewfront _output)) "Undefined" self 0))

(event EventOnEquipped
  ;[1 1 1] 여기서 블랙홀, 실드 생성 혹은 삭제
)

(event EventOnUnEquipped
  ;[1 1 1] 여기서 블랙홀, 실드 생성 혹은 삭제
)

(event EventEndSubWeapon
  ;[1 1 1] 여기서 블랙홀, 실드 생성 혹은 삭제
)

(fn ConstructionScript)

(fn GetSpawnFrontVector
  (params (ActorFrontOrViewFront :type Boolean%20%28by%20ref%29))
  (bind _ascharacter (CallFunction|GetOwnertoCharacter))
  (bind _returnvalue (Transformation|GetActorForwardVector _ascharacter))
  (bind _returnvalue_2 (Pawn|GetController _ascharacter))
  (bind _mesh (Variables|/Script/Engine.Character|GetMesh _ascharacter))
  (bind _returnvalue_3 (Pawn|GetControlRotation _returnvalue_2 :!class /Script/Engine.Controller))
  (bind _returnvalue_4 (* _returnvalue 5e+01))
  (bind _returnvalue_5 (Transformation|GetSocketLocation _mesh "Spine_03"))
  (bind _returnvalue_6 (+ _returnvalue_5 _returnvalue_4))
  (if ActorFrontOrViewFront
    (return (Math|Transform|MakeTransform _returnvalue_6 (Math|Rotator|MakeRotator 0.0 0.0 (.Yaw (Math|Rotator|BreakRotator _returnvalue_3)))))
    (else
      (return (Math|Transform|MakeTransform _returnvalue_6 _returnvalue_3)))))

(fn SetSubWeaponIcon
  (params (currentIndex :type Integer) (SubWeaponContainerWidget :type WB%20Sub%20Weapon%20Container%20Object%20Reference%20%28by%20ref%29))
  (bind _subweaponitems (Variables|Default|GetSubWeaponItems))
  (bind _returnvalue (Utilities|Array|Length _subweaponitems))
  (for _index (range 0 (- _returnvalue 1))
    (Default|SetSlotIcon SubWeaponContainerWidget (+ _index currentIndex) (.icontexture (Utilities|Array|Get(acopy) _subweaponitems _index))))
  (return _returnvalue))