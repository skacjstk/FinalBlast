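; One-way shield sub-weapon actor that exists for a set duration and decides which projectiles and line traces may pass through it.
; On BeginPlay it sizes the shield mesh and starts a duration-scaled timeline that drives material opacity, then destroys the actor.
; Pathability checks switch on collision object type and use a dot product with the shield's forward vector, passing only non-positive results for direction-tested cases.
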(event Custom|ItemStart_1
  (Components|Timeline|SetPlayRate (Variables|Default|GetShieldDuration) (/ 1.0 (Variables|Default|GetDuration)))
  (bind _shieldopacityalpha (Timeline|ShieldDuration PlayFromStart)
    (:Update
      (Rendering|Material|SetScalarParameterValueonMaterials (Variables|Default|GetShield) "Opacity" _shieldopacityalpha))
    (:Finished
      (Actor|DestroyActor))))

(event EventBeginPlay
  (CallFunction|SetShieldSize "10.000000,600.000000,300.000000")
  (CallFunction|ItemStart1))

(event Collision|EventActorBeginOverlap
  (params (OtherActor :type Actor%20Object%20Reference)))

(event EventSetShieldSize
  (params (Size :type Vector :default "0, 0, 0"))
  (Transformation|SetWorldScale3D (Variables|Default|GetShield) (* Size 0.01)))

(fn ConstructionScript
  (Transformation|SetWorldScale3D (Variables|Default|GetShield) (* (Variables|Default|GetShieldSize) 0.01)))

(fn IsPathableWall
  (params (Projectile :type Actor%20Object%20Reference) (ProjectileCollision :type Primitive%20Component%20Object%20Reference))
  (if (not (Class|ActorComponent|IsBeingDestroyed ProjectileCollision))
    (switch Utilities|FlowControl|Switch|SwitchonECollisionChannel (Collision|GetCollisionObjectType ProjectileCollision)
      (:ECC_WorldStatic
        _)
      (:ECC_WorldDynamic
        (bind _shieldvector (CallFunction|GetCompareVector :!label _label))
        (return (<= (Math|Vector|DotProduct _shieldvector (Transformation|GetVelocity Projectile)) 0.0)))
      (:ECC_Pawn
        _)
      (:ECC_Visibility
        (return false))
      (:ECC_Camera
        (return false))
      (:ECC_PhysicsBody
        _)
      (:ECC_Vehicle
        _)
      (:ECC_Destructible
        _)
      (:ECC_GameTraceChannel1
        (return false))
      (:ECC_GameTraceChannel2
        (return false))
      (:ECC_GameTraceChannel3
        (goto _label)))
    (return true)))

(fn GetCompareVector
  (return (Math|Vector|GetForwardVector (Variables|Default|GetShield))))

(fn IsPathableLinetrace
  (params (AimDirection :type Vector%20%28by%20ref%29 :default "0, 0, 0"))
  (bind _shieldvector (CallFunction|GetCompareVector))
  (return (<= (Math|Vector|DotProduct _shieldvector AimDirection) 0.0)))