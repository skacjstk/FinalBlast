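; Throwable grenade item that launches on a timer fuse and explodes with radial burning damage.
; Collision stays off until RefreshExplosionTimer enables physics, detaches the grip as a separate simulated piece, and throws both along the given camera vector with added upward lift.
; After the delay, it applies falloff damage at the capsule, plays explosion sound and particles, then destroys itself.
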(event Custom|Test
  (bind _capsule (Variables|Default|GetCapsule))
  (bind _returnvalue (Transformation|GetWorldLocation _capsule))
  ;[1 1 1] AnyDamage 라면 이 데미지에 대한 걸 받아낼 수 있구나
  (Class|GameplayStatics|ApplyRadialDamagewithFalloff 1e+02 1e+01 _returnvalue 2e+02 1e+03 1.0 "/Game/Components/DamageType/BurningDamage.BurningDamage_C" 0 self (Game|GetInstigatorController) "ECC_Visibility")
  (Audio|PlaySoundatLocation "/Game/Sounds/Wave/Weapon/Grenade/Grenade_Explosion.Grenade_Explosion" _returnvalue "0, 0, 0" 1.0 1.0 0.0 0 0 0)
  ;[1 1 1] 이거때문에 가려지는건 아닌..거 같아, 6번에 문제가 있음
  (Rendering|SetVisibility (Variables|Default|GetCapsule) false true)
  (Effects|SpawnEmitteratLocation "/Game/Explosions/Particles/P_ImpactExplosion2.P_ImpactExplosion2" _returnvalue)
  (Actor|DestroyActor))

(event Custom|RefreshExplosionTimer
  (params (CameraVector :type Vector))
  (bind _velocity (Variables|Default|GetVelocity))
  (bind _capsule (Variables|Default|GetCapsule))
  (Collision|SetCollisionEnabled (Variables|Default|GetCapsule) "QueryAndPhysics")
  (Physics|SetSimulatePhysics (Variables|Default|GetCapsule) true)
  (CallFunction|DetachGrip)
  (Class|PrimitiveComponent|SetAllPhysicsLinearVelocity _capsule (* CameraVector _velocity) false)
  (Class|PrimitiveComponent|SetAllPhysicsLinearVelocity _capsule (Math|Vector|MakeVector 0.0 0.0 (* _velocity 0.5)) true)
  (Utilities|Time|SetTimerbyEvent (delegate Custom|Test) (Variables|Default|GetExplosionDelay)))

(event Custom|DetachGrip
  (bind _grip (Variables|Default|GetGrip))
  (Transformation|DetachFromComponent _grip "KeepWorld" "KeepWorld" "KeepWorld" true)
  (Physics|SetSimulatePhysics _grip true))

(event EventBeginPlay
  (|CallParentFunction)
  (Collision|SetCollisionEnabled (Variables|Default|GetCapsule) "NoCollision"))

(event EventTick
  (params (DeltaSeconds :type Float%20%28single-precision%29)))

(fn ConstructionScript
  (|CallParentFunction))