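; BP_BlackHole is a sub-weapon projectile that becomes a temporary black hole on overlapping anything but its owner, respecting BP_OneWayShield pathability.
; Activation stops movement, swaps particles and starts a timeline scaling the pull radius over Duration, after which the actor is destroyed.
; A looping per-frame-rate timer runs debug-drawn sphere traces, launching non-owner Characters toward the center and pulling physics bodies with mass-scaled negative radial impulses.
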(event OnComponentBeginOverlap(Box)
  (params (OverlappedComponent :type Primitive%20Component%20Object%20Reference) (OtherActor :type Actor%20Object%20Reference) (OtherComp :type Primitive%20Component%20Object%20Reference) (OtherBodyIndex :type Integer) (bFromSweep :type Boolean) (SweepResult :type Hit%20Result%20Structure%20%28by%20ref%29))
  (bind _as_character (CallFunction|GetOwnertoCharacter))
  (bind _returnvalue (!= OtherActor _as_character))
  (bind _asbp_one_way_shield (Utilities|Casting|CastToBP_OneWayShield OtherActor)
    (:then
      (bind _cannotpath (Default|IsPathableWall _asbp_one_way_shield self (Variables|Default|GetBox)))
      ;[1 1 1] 자기자신 제외 충돌시, 블랙홀 발동
      (if (and _returnvalue _cannotpath)
        (CallFunction|ActiveBlackHole :!label _label)))
    (:CastFailed
      (if _returnvalue
        (goto _label)))))

(event Custom|SetCurrentRadius
  ;[1 1 1] 1/Duration 만큼 CurrentRadius 를 1~0 scale 로 조정함.
  (Variables|Default|SetcurrentRadius (Variables|Default|GetRadius))
  (Components|Timeline|SetPlayRate (Variables|Default|GetRadiusTimeline) (/ 1.0 (Variables|Default|GetDuration)))
  (bind _radiusalpha (Timeline|RadiusTimeline PlayFromStart)
    (:Update
      (Variables|Default|SetcurrentRadius (Math|Float|Lerp 0.0 (Variables|Default|GetRadius) _radiusalpha)))))

(event Custom|ActiveBlackHole
  (bind _blackholeonparticle (Variables|Default|GetBlackHoleOnParticle))
  ;[1 1 1] 블랙홀 발생
  (CallFunction|SetParticle false (Variables|Default|GetProjectileParticle))
  (if (not (Variables|Default|GetCoolDown))
    (Variables|Default|SetCoolDown true)
    (CallFunction|SetCurrentRadius) ; 타이머 설정 전에 호출해야함
    (bind _returnvalue (Utilities|Time|SetTimerbyEvent (delegate Custom|Explosion) 0.016 true)) ; 필요한 순간
    (Niagara|ResetSystem _blackholeonparticle)
    (Rendering|SetVisibility _blackholeonparticle true false)
    (Components|Activation|SetActive (Variables|Default|GetBlackHoleOnParticle) true false)
    (Components|Movement|StopMovementImmediately (Variables|Default|GetProjectileMovement))
    ;[1 1 1] 블랙홀 소멸
    (Utilities|FlowControl|Delay (Variables|Default|GetDuration))
    (Utilities|Time|ClearandInvalidateTimerbyHandle _returnvalue)
    (Actor|DestroyActor)))

(event Custom|Explosion
  (bind _returnvalue (Transformation|GetActorLocation))
  (bind _returnvalue_2 (Transformation|GetActorLocation))
  ;[1 1 1] 기본 객체 빨아들이기
  (bind _outhits (Collision|MultiSphereTraceForObjects _returnvalue _returnvalue (Variables|Default|GetcurrentRadius) (Utilities|Array|MakeArray "ObjectTypeQuery2" "ObjectTypeQuery4" "ObjectTypeQuery3") false 0 "ForDuration" true "(R=1.000000,G=0.000000,B=0.000000,A=1.000000)" "(R=0.000000,G=1.000000,B=0.000000,A=1.000000)" 0.016))
  (for _array_element _outhits
    (bind _ascharacter (Utilities|Casting|CastToCharacter (.HitActor (Collision|BreakHitResult _array_element)))
      (:then
        (if (not (== _ascharacter (CallFunction|GetOwnertoCharacter))) ; 시전자 제외
          (Character|LaunchCharacter _ascharacter (- _returnvalue_2 (Transformation|GetActorLocation _ascharacter)) false false)))
      (:CastFailed
        (if (Physics|IsSimulatingPhysics (.HitComponent (Collision|BreakHitResult _array_element)) "None")
          (Physics|AddRadialImpulse (.HitComponent (Collision|BreakHitResult _array_element)) _returnvalue_2 5e+02 (/ -5e+05 (Physics|GetMass (.HitComponent (Collision|BreakHitResult _array_element)))) "RIF_Constant" false))))))

(event EventBeginPlay
  (bind _radius (Variables|Default|GetRadius))
  (bind _returnvalue (* _radius 0.75))
  ;[1 1 1] BeginPlay: 파티클 초기세팅
  (Niagara|ResetSystem (Variables|Default|GetBlackHoleOnParticle))
  (CallFunction|SetParticle false (Variables|Default|GetBlackHoleOnParticle))
  (CallFunction|SetParticle true (Variables|Default|GetProjectileParticle))
  (Effects|Components|ParticleSystem|SetFloatParameter (Variables|Default|GetBlackHoleOnParticle) "Duration" (Variables|Default|GetDuration))
  (Effects|Components|ParticleSystem|SetFloatParameter (Variables|Default|GetBlackHoleOnParticle) "ParticleRadius" _returnvalue)
  (Effects|Components|ParticleSystem|SetVectorParameter (Variables|Default|GetBlackHoleOnParticle) "RingScale" (Math|Conversions|ToVector(Float) _returnvalue)))

(fn ConstructionScript)

(fn SetParticle
  (params (bool :type Boolean) (NewParam :type Niagara%20Component%20Object%20Reference%20%28by%20ref%29))
  (Rendering|SetVisibility NewParam bool false)
  (Components|Activation|SetActive NewParam bool false))