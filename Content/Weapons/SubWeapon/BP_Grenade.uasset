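; Grenade sub-weapon that lets an idle owner character throw a timed grenade when the sub-weapon can be used.
; Starting it plays the Grenade montage and spawns a grenade actor attached to the hand socket, destroyed if interrupted before the throw.
; The montage notify consumes a use, refreshes regeneration, detaches the grenade and starts its fuse with player 0's camera forward vector.
; A radial burning-damage Test event remains, its timer unwired.
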(event Custom|Test
  (bind _ascharacter (CallFunction|GetOwnertoCharacter))
  (bind _returnvalue (Transformation|GetActorLocation _ascharacter))
  ;[1 1 1] AnyDamage 라면 이 데미지에 대한 걸 받아낼 수 있구나
  (Class|GameplayStatics|ApplyRadialDamagewithFalloff 2e+01 1e+01 _returnvalue 1e+02 3e+02 1.0 "/Game/Components/DamageType/BurningDamage.BurningDamage_C" (Utilities|Array|MakeArray _ascharacter) self (Game|GetInstigatorController) "ECC_Visibility")
  (Audio|PlaySoundatLocation "/Game/Sounds/Wave/Weapon/Grenade/Grenade_Explosion.Grenade_Explosion" "0, 0, 0" "0, 0, 0" 1.0 1.0 0.0 0 0 0)
  (Effects|SpawnEmitteratLocation "/Game/Explosions/Particles/P_ImpactExplosion6.P_ImpactExplosion6" _returnvalue))

(event EventBeginPlay
  (|CallParentFunction))

(event EventReleaseSubWeapon
  (params (SelectedItemIndex :type Integer)))

(event EventStartSubweapon
  (params (SelectedItemIndex :type Integer))
  (bind _ascharacter (CallFunction|GetOwnertoCharacter))
  (bind _iswproperty (Variables|Default|GetISWProperty))
  (bind _subweaponcomponent (Variables|Default|GetSubWeaponComponent))
  (bind (_itemname _hascooltime _hasuselimit _cooltime _inituselimit) (Utilities|Struct|BreakFISWProperty _iswproperty))
  (bind _canuse (CallFunction|CheckCanUseSubWeapon _iswproperty))
  (if _canuse
    (bind _result (Class|IState|IsStateIdling(Message) _ascharacter))
    (if _result
      (bind (_animmontage _findsuccess) (Class|IState|GetAnimMontage(Message) _ascharacter "Grenade"))
      (if _findsuccess
        (Animation|Montage|PlayMontage (Variables|/Script/Engine.Character|GetMesh _ascharacter) _animmontage
          (:then
            (bind _returnvalue (Game|SpawnActorfromClass "/Game/Weapons/SubWeapon/SubWeapons/BP_ItemGrenade.BP_ItemGrenade_C" (Math|Transform|MakeTransform "0, 0, 0" "0, 0, 0" "0.500000,0.500000,0.500000") "AlwaysSpawn" (CallFunction|GetOwnertoCharacter) (Pawn|GetControlledPawn (Game|GetInstigatorController))))
            ;[1 1 1] 충돌체를 끈 채로 시작(비긴플레이) + AttachToComponent
            (bind _output_get (Variables|Default|SetItemGrenade _returnvalue))
            (Transformation|AttachComponentToComponent _output_get (Variables|/Script/Engine.Character|GetMesh (CallFunction|GetOwnertoCharacter)) "Hand_Grenade" "KeepRelative" "KeepRelative" "KeepRelative" false)
            (Variables|Default|SetIsGrenadeThrowed false))
          (:OnInterrupted
            (if (not (Variables|Default|GetIsGrenadeThrowed))
              (Actor|DestroyActor (Variables|Default|GetItemGrenade))))
          (:OnNotifyBegin
            (Variables|Default|SetIsGrenadeThrowed true)
            (CallFunction|UseSubWeapon _iswproperty)
            (Default|InitMemberValue _subweaponcomponent SelectedItemIndex -1 false)
            (Default|RefreshRegenTimer _subweaponcomponent _cooltime _hasuselimit _inituselimit)
            ;[1 1 1] 이제 실물 Grenade를 쉭 던지면 됨
            (Transformation|DetachFromActor (Variables|Default|GetItemGrenade) "KeepWorld" "KeepWorld" "KeepWorld")
            (Variables|/Game/Weapons/SubWeapon/SubWeapons/BP_ItemGrenade.BP_ItemGrenade_C|SetExplosionDelay (Variables|Default|GetItemGrenade) 3.0)
            (Default|RefreshExplosionTimer (Variables|Default|GetItemGrenade) (Transformation|GetActorForwardVector (Game|GetPlayerCameraManager 0)))))))))

(fn ConstructionScript
  (|CallParentFunction))