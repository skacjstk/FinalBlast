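; BP_SubWeapon is a base Blueprint for sub-weapons, with empty start, end, equip and unequip events as virtual hooks.
; Helper functions walk the owner chain, casting its owner to BP_SubWeaponForEquip and that object's owner to Character.
; SetSubWeaponIcon writes its icon into a given slot of the container widget, while GetSubWeaponItems is an empty stub.
; BeginPlay initializes the container index.
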(event Custom|OnUnEquipped
  ;[1 1 1] 가상
)

(event Custom|OnEquipped
  ;[1 1 1] 가상
)

(event Custom|StartSubweapon
  ;[1 1 1] 가상
)

(event Custom|EndSubWeapon
  ;[1 1 1] 가상
)

(event EventBeginPlay
  (Variables|Default|SetInitialContainerIndex 1))

(fn ConstructionScript)

(fn GetOwnertoSubWeaponforEquip
  (bind _asbp_sub_weapon_for_equip (Utilities|Casting|CastToBP_SubWeaponForEquip (Components|GetOwner)))
  (return _asbp_sub_weapon_for_equip))

(fn GetOwnertoCharacter
  (bind _ascharacter (Utilities|Casting|CastToCharacter (Components|GetOwner (CallFunction|GetOwnertoSubWeaponforEquip))))
  (return _ascharacter))

(fn GetSubWeaponItems)

(fn SetSubWeaponIcon
  (params (currentIndex :type Integer) (SubWeaponContainerWidget :type WB%20Sub%20Weapon%20Container%20Object%20Reference%20%28by%20ref%29))
  (Default|SetSlotIcon SubWeaponContainerWidget currentIndex (Variables|Default|GetIcon))
  (return 1))