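; Equippable sub-weapon that holds spawner actors and forwards attack and equip calls to the currently selected one.
; On BeginPlay it spawns a BP_SpawnerSubWeapon, records each container's slot count and fills the owner's icon widget through IWeapon.
; FocusSubWeapon maps a flat index across those counts to a container and item within it.
; Switching containers unequips the old sub-weapon and equips the new one.
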(event Custom|FocusSubWeapon
  (params (New%20Index :type Integer))
  ;[1 1 1] 포커싱할 Item 결정
  (bind _result (Math|Integer|IncrementInt New%20Index)
    (:%20%20
      (Variables|Default|SetFindFocusElemIndex _result)
      (bind (_array_element _array_index) (Utilities|Array|ForEachLoopwithBreak (Variables|Default|GetSubWeaponConainerNum) :!label _label)
        (:LoopBody
          (if (>= _array_element (Variables|Default|GetFindFocusElemIndex))
            (Variables|Default|SetSelectedIndex _array_index)
            (goto _label Break)
            (else
              (Variables|Default|SetFindFocusElemIndex (- (Variables|Default|GetFindFocusElemIndex) _array_element)))))
        (:Completed
          (bind _asbp_spawner_sub_weapon (Utilities|Casting|CastToBP_SpawnerSubWeapon (Utilities|Array|Get(acopy) (Variables|Default|GetSubWeaponContainer) (Variables|Default|GetSelectedIndex)))
            (:then
              ;;[1 1 1] 추가 현재아이템 설정
              (CallFunction|SetCurrentSubWeapon _asbp_spawner_sub_weapon)
              (bind _output_get (Variables|/Game/Weapons/SubWeapon/SubWeapons/BP_SpawnerSubWeapon.BP_SpawnerSubWeapon_C|SetcurrentItem _asbp_spawner_sub_weapon (Math|Integer|%(Integer) (- (Variables|Default|GetFindFocusElemIndex) 1) (Utilities|Array|Length (Variables|/Game/Weapons/SubWeapon/SubWeapons/BP_SpawnerSubWeapon.BP_SpawnerSubWeapon_C|GetSubWeaponItems _asbp_spawner_sub_weapon))))))
            (:CastFailed
              (CallFunction|SetCurrentSubWeapon _asbp_spawner_sub_weapon))))))))

(event EventBeginPlay
  (|CallParentFunction)
  (Utilities|FlowControl|Sequence
    (:then_2
      (bind _returnvalue (Game|SpawnActorfromClass "/Game/Weapons/SubWeapon/SubWeapons/BP_SpawnerSubWeapon.BP_SpawnerSubWeapon_C" (Math|Transform|MakeTransform "0, 0, 0") "Undefined" self 0))
      (bind _output_get (Variables|Default|SetSpawnSubWeapon _returnvalue))
      (Utilities|Array|Add (Variables|Default|GetSubWeaponContainer) _output_get))
    (:then_3
      ;[1 1 1] BP_Weapon 상속받은 이 무기가 가진 무기별 Container Index의 총합
      (for _array_element (Variables|Default|GetSubWeaponContainer)
        (Utilities|Array|Add (Variables|Default|GetSubWeaponConainerNum) (Variables|/Game/Weapons/SubWeapon/BP_SubWeapon.BP_SubWeapon_C|GetInitialContainerIndex _array_element))
        (Variables|Default|SetMaxEquipIndex (+ (Variables|/Game/Weapons/SubWeapon/BP_SubWeapon.BP_SubWeapon_C|GetInitialContainerIndex _array_element) (Variables|Default|GetMaxEquipIndex))))
      ;[1 1 1] 현재무기 설정
      (Variables|Default|SetCurrentSubWeapon (Variables|Default|GetSpawnSubWeapon)))
    (:then_4
      (|SetSubWeaponIcon))))

(fn ConstructionScript
  (|CallParentFunction))

(fn Attack
  (bind _currentsubweapon (Variables|Default|GetCurrentSubWeapon))
  (|CallParentFunction)
  (if (Utilities|IsValid _currentsubweapon)
    (if true
      (Default|StartSubweapon _currentsubweapon))))

(fn EndAttack
  (|CallParentFunction)
  (Default|EndSubWeapon (Variables|Default|GetCurrentSubWeapon)))

(fn OnEquipped
  (bind _currentsubweapon (Variables|Default|GetCurrentSubWeapon))
  (Utilities|IsValid _currentsubweapon
    (:Is%20Valid
      (Default|OnEquipped _currentsubweapon))))

(fn OnUnEquipped
  (bind _currentsubweapon (Variables|Default|GetCurrentSubWeapon))
  (Utilities|IsValid _currentsubweapon
    (:Is%20Valid
      (Default|OnUnEquipped _currentsubweapon))))

(fn SetCurrentSubWeapon
  (params (New%20SubWeapon :type BP%20Sub%20Weapon%20Object%20Reference))
  (if (!= New%20SubWeapon (Variables|Default|GetCurrentSubWeapon))
    (bind _currentsubweapon (Variables|Default|GetCurrentSubWeapon)
      (:then
        (Default|OnUnEquipped _currentsubweapon))
      (:else
        _))
    (bind _new_subweapon (LocalVariables|GetNew%20SubWeapon)
      (:then
        (Variables|Default|SetCurrentSubWeapon _new_subweapon)
        (CallFunction|OnEquipped))
      (:else
        (Variables|Default|SetCurrentSubWeapon 0)))))