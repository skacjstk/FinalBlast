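; Thunder ball magic projectile that deals damage and shows a thunder impact particle on what it overlaps.
; Sphere overlaps ignore the owner of the magic and pass the WeaponDamageComponent's single damage to SendThrowDamage.
; A BP_OneWayShield is hit only when its IsPathableWall check returns true for this projectile and sphere.
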(event OnComponentBeginOverlap(Sphere)
  (params (OverlappedComponent :type Primitive%20Component%20Object%20Reference) (OtherActor :type Actor%20Object%20Reference) (OtherComp :type Primitive%20Component%20Object%20Reference) (OtherBodyIndex :type Integer) (bFromSweep :type Boolean) (SweepResult :type Hit%20Result%20Structure%20%28by%20ref%29))
  (bind _asbp_skill_throw (CallFunction|GetOwnertoMagic))
  (bind _returnvalue (Components|GetOwner _asbp_skill_throw))
  (bind _returnvalue_2 (!= OtherActor _returnvalue))
  (bind _asbp_one_way_shield (Utilities|Casting|CastToBP_OneWayShield OtherActor)
    (:then
      (bind _cannotpath (Default|IsPathableWall _asbp_one_way_shield self (Variables|Default|GetSphere)))
      (if (and _cannotpath _returnvalue_2)
        (bind _returnvalue_3 (Default|GetSingleDamage (Variables|Default|GetWeaponDamageComponent) :!label _label))
        (CallFunction|SendThrowDamage OtherActor "/Game/Particles/P_Impact_ThunderBall.P_Impact_ThunderBall" "0.000000,0,0" "0.200000,0.200000,0.200000" _returnvalue_3)))
    (:CastFailed
      (if _returnvalue_2
        (goto _label)))))

(event EventBeginPlay
  (|CallParentFunction))

(fn ConstructionScript)