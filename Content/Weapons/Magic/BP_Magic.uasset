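; BP_Magic is a magic weapon that delegates attacks and equip events to a current skill actor.
; On BeginPlay it spawns Heal, Warp and Throw skill actors, attaches them to the owning character's mesh and selects Heal.
; Attack sets the spelling state and calls Spell when allowed; EndAttack returns to idle and calls EndSpell.
; SetCurrentSkill switches skills, unequipping the old one and equipping the new one.
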(event EventBeginPlay
  (|CallParentFunction)
  (Utilities|FlowControl|Sequence
    (:then_0
      (|SpawnHeal))
    (:then_1
      (|SpawnWarp))
    (:then_2
      (|SpawnThrow))
    (:then_3
      (Variables|Default|SetCurrentSkill (Variables|Default|GetHeal)))))

(event Collision|EventActorBeginOverlap
  (params (OtherActor :type Actor%20Object%20Reference))
  (|CallParentFunction OtherActor) ; 지금 이 노드는 비활성 상태입니다. \n핀을 끌어서 다른 노드를 연결하면 활성화됩니다.
)

(event EventTick
  (params (DeltaSeconds :type Float%20%28single-precision%29))
  (|CallParentFunction DeltaSeconds) ; 지금 이 노드는 비활성 상태입니다. \n핀을 끌어서 다른 노드를 연결하면 활성화됩니다.
)

(fn ConstructionScript
  (|CallParentFunction))

(fn Attack
  (|CallParentFunction)
  (if (and (CallFunction|CanAttack) (Utilities|IsValid (Variables|Default|GetCurrentSkill)))
    (CallFunction|SetStateSpelling)
    (Default|Spell (Variables|Default|GetCurrentSkill))))

(fn EndAttack
  (|CallParentFunction)
  (CallFunction|SetStateIdling)
  (Default|EndSpell (Variables|Default|GetCurrentSkill)))

(fn OnEquipped
  (Utilities|IsValid (Variables|Default|GetCurrentSkill)
    (:Is%20Valid
      (Default|OnEquipped (Variables|Default|GetCurrentSkill)))))

(fn OnUnEquipped
  (Utilities|IsValid (Variables|Default|GetCurrentSkill)
    (:Is%20Valid
      (Default|OnUnEquipped (Variables|Default|GetCurrentSkill))
      (Development|PrintString "마법모드 꺼짐" true false))))

(fn SetCurrentSkill
  (params (New%20Skill :type BP%20Skill%20Object%20Reference))
  (if (!= New%20Skill (Variables|Default|GetCurrentSkill))
    (bind _currentskill (Variables|Default|GetCurrentSkill)
      (:then
        (Default|OnUnEquipped _currentskill))
      (:else
        _))
    (bind _new_skill (LocalVariables|GetNew%20Skill)
      (:then
        (bind _output_get (Variables|Default|SetCurrentSkill _new_skill))
        (Default|OnEquipped _output_get))
      (:else
        (Variables|Default|SetCurrentSkill 0)))))