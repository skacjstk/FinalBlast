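; BP_ThrowItem is the actor for items thrown by magic throw skills, with a limited lifespan and helpers for hits and wall checks.
; It climbs the owner chain through BP_SkillThrow to BP_Magic, which applies damage after an impact emitter spawns, then destroys itself a frame later.
; IsPathableWall decides passability by collision object type, letting one-way walls through when their direction vector dotted with the item's velocity is positive.
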(event Custom|DestroyDelayed
  (Utilities|FlowControl|Delay (Utilities|Time|GetWorldDeltaSeconds))
  (Actor|DestroyActor))

(event EventBeginPlay
  (Actor|SetLifeSpan (Variables|Default|GetLifeSpan)))

(event Collision|EventActorBeginOverlap
  (params (OtherActor :type Actor%20Object%20Reference)))

(event EventTick
  (params (DeltaSeconds :type Float%20%28single-precision%29)))

(fn ConstructionScript)

(fn GetOwnertoThrow
  (bind _asbp_skill_throw (Utilities|Casting|CastToBP_SkillThrow (Components|GetOwner)))
  (return _asbp_skill_throw))

(fn GetOwnertoMagic
  (bind _asbp_magic (Utilities|Casting|CastToBP_Magic (Components|GetOwner (CallFunction|GetOwnertoThrow))))
  (return _asbp_magic))

(fn SendThrowDamage
  (params (OtherActor :type Actor%20Object%20Reference) (ImpactParticle :type Particle%20System%20Object%20Reference) (ImpactParticleOffset :type Vector :default "0.000000,0,0") (ImpactParticleScale :type Vector :default "1.000000,1.000000,1.000000") (Damage :type Float%20%28single-precision%29) (DamageType :type Damage%20Type%20Class%20Reference))
  (Effects|SpawnEmitteratLocation ImpactParticle (+ ImpactParticleOffset (Transformation|GetActorLocation)) (Math|Rotator|FindLookatRotation (Transformation|GetActorLocation (Components|GetOwner (CallFunction|GetOwnertoMagic))) (Transformation|GetActorLocation OtherActor)) ImpactParticleScale)
  (Default|SendDamage (CallFunction|GetOwnertoMagic) OtherActor Damage false DamageType)
  (CallFunction|DestroyDelayed))

(fn IsPathableWall
  (params (Other%20Actor :type Actor%20Object%20Reference%20%28by%20ref%29) (Other%20Comp :type Primitive%20Component%20Object%20Reference%20%28by%20ref%29))
  (if (not (Class|ActorComponent|IsBeingDestroyed Other%20Comp))
    (switch Utilities|FlowControl|Switch|SwitchonECollisionChannel (Collision|GetCollisionObjectType Other%20Comp)
      (:ECC_WorldStatic
        _)
      (:ECC_WorldDynamic
        _)
      (:ECC_Pawn
        _)
      (:ECC_Visibility
        (return true))
      (:ECC_Camera
        (return true))
      (:ECC_PhysicsBody
        _)
      (:ECC_Vehicle
        _)
      (:ECC_Destructible
        _)
      (:ECC_GameTraceChannel1
        (return true))
      (:ECC_GameTraceChannel2
        (Utilities|IsValid Other%20Actor
          (:Is%20Valid
            (bind _shieldvector (Class|IOneWayShield|GetCompareVector(Message) Other%20Actor))
            (return (> (Math|Vector|DotProduct _shieldvector (Transformation|GetVelocity)) 0.0))))))
    (return false)))