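; Warp magic skill that teleports its owner to the world-static surface point under the mouse cursor.
; While equipped, Tick moves a decal and mesh marker to the cursor hit, aligns the decal to the surface normal, and hides both on a miss.
; Spell stores the target and plays the "Warp" data table row's montage, or ends the attack without a hit.
; A notify-called Warp event then moves the owner slightly above the target.
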(event Custom|Warp
  (bind _warplocation (Variables|Warp|GetWarpLocation))
  (bind (_x _y _z) (Math|Vector|BreakVector _warplocation))
  ;[1 1 1] 워프
  (if (Variables|Warp|GetCanWarp)
    (Variables|Warp|SetCanWarp false)
    (Transformation|SetActorLocation (CallFunction|GetOwnertoCharacter) (Math|Vector|MakeVector _x _y (+ _z 5e+01)) false false)))

(event EventTick
  (params (DeltaSeconds :type Float%20%28single-precision%29))
  (bind _decal (Variables|Default|GetDecal))
  (bind (_location _impactpoint) (Utilities|GetCursorLocation)
    (:True
      (Transformation|SetWorldLocation _decal _location false false)
      (Transformation|SetWorldRotation _decal (Math|Conversions|RotationFromXVector _impactpoint) false false))
    (:False
      (Rendering|SetVisibility _decal false false))))

(event EventBeginPlay
  (|CallParentFunction)
  ;[1 1 1] 딱 한줄 가져옴(모션이 1개라서 이게 더 간단)
  (bind _returnvalue (Utilities|GetDataTableRow (Variables|Default|GetDataTable) "Warp")
    (:then
      (Variables|Default|SetMagicData _returnvalue)
      (Rendering|SetVisibility (Variables|Default|GetDecal) false false))))

(event EventOnEquipped
  (|CallParentFunction)
  (Variables|Default|SetEquippedSkill true)
  (Rendering|SetVisibility (Variables|Default|GetDecal) true false)
  (Actor|Tick|SetActorTickEnabled true))

(event EventSpell
  (bind _magicdata (Variables|Default|GetMagicData))
  (bind (_skilltype _montage _playrate _startsection _canmove) (Utilities|Struct|BreakFMagicData _magicdata))
  (|CallParentFunction)
  (bind _location (Utilities|GetCursorLocation)
    (:True
      (Variables|Warp|SetCanWarp true)
      (Variables|Warp|SetWarpLocation _location)
      (Default|SetCanMove (CallFunction|GetOwnertoMagic) _canmove)
      (Animation|PlayAnimMontage (CallFunction|GetOwnertoCharacter) _montage _playrate _startsection) ; 얘 자체에 뭔가 있어서 못움직였다가 움직여짐
    )
    (:False
      (Default|EndAttack (CallFunction|GetOwnertoMagic))
      (Variables|Warp|SetCanWarp false))))

(event EventEndSpell
  (|CallParentFunction)
  (Default|SetCanMove (CallFunction|GetOwnertoMagic) true))

(event EventOnUnEquipped
  (|CallParentFunction)
  (Variables|Default|SetEquippedSkill false)
  (Rendering|SetVisibility (Variables|Default|GetDecal) false false)
  (Actor|Tick|SetActorTickEnabled false))

(fn ConstructionScript
  (|CallParentFunction))