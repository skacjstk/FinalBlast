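; BP_Skill is the base Blueprint for magic skills, owned by a BP_Magic actor whose owner is a Character.
; On BeginPlay it picks its DataTable from the character's skeletal mesh name, covering Mannequin, Vanguard and Twin Blast.
; Spell and EndSpell are empty virtual hooks for subclasses.
; Equip and unequip both re-enable movement and return the magic to idle through owner-chain helper getters.
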(event Custom|Spell)

(event Custom|EndSpell)

(event Custom|OnUnEquipped
  (bind _asbp_magic (CallFunction|GetOwnertoMagic))
  (Default|SetCanMove _asbp_magic true)
  (Default|SetStateIdling _asbp_magic))

(event Custom|OnEquipped
  (bind _asbp_magic (CallFunction|GetOwnertoMagic))
  (Default|SetCanMove _asbp_magic true)
  (Default|SetStateIdling _asbp_magic))

(event EventBeginPlay
  ;[1 1 1] 비긴플레이: DataTable 설정
  (switch name (Utilities|String|StringToName (Utilities|GetObjectName (Variables|/Script/Engine.SkinnedMeshComponent|GetSkeletalMesh (Variables|/Script/Engine.Character|GetMesh (CallFunction|GetOwnertoCharacter)))))
    (:SK_Mannequin
      (Variables|Default|SetDataTable "/Game/DataTables/Mannequin/DT_Magic.DT_Magic"))
    (:Vanguard_By_T__Choonyung
      (Variables|Default|SetDataTable "/Game/DataTables/Vanguard/DT_MagicVanguard.DT_MagicVanguard"))
    (:TwinBlast
      (Variables|Default|SetDataTable "/Game/DataTables/TwinBlast/DT_MagicTwinBlast.DT_MagicTwinBlast"))))

(fn ConstructionScript)

(fn GetOwnertoMagic
  (bind _asbp_magic (Utilities|Casting|CastToBP_Magic (Components|GetOwner)))
  (return _asbp_magic))

(fn GetOwnertoCharacter
  (bind _ascharacter (Utilities|Casting|CastToCharacter (Components|GetOwner (CallFunction|GetOwnertoMagic))))
  (return _ascharacter))