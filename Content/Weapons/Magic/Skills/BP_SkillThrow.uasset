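; Throwing skill that lets its owning character hurl a selectable item, switching BP_Player to a side camera while equipped.
; BeginPlay loads the single "Throw" DataTable row, which drives the montage and movement permission in Spell until EndSpell re-enables movement.
; BeginThrow spawns the current item's class at the Hand_Throw socket, aimed by player 0's control rotation.
; SetCurrentItem selects the ThrowItems entry by class and updates the attached particle.
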(event Custom|BeginThrow
  ;[1 1 1] 실제 객체 생성
  (Game|SpawnActorfromClass (.throwitemclass (Utilities|Array|Get(acopy) (Variables|Default|GetThrowItems) (Variables|Default|GetCurrentItem))) (Math|Transform|MakeTransform (Transformation|GetSocketLocation (Variables|/Script/Engine.Character|GetMesh (CallFunction|GetOwnertoCharacter)) "Hand_Throw") (Pawn|GetControlRotation (Game|GetPlayerController 0) :!class /Script/Engine.Controller) (Variables|Default|GetparticleScale)) "Undefined" self (CallFunction|GetOwnertoCharacter)))

(event EventBeginPlay
  (|CallParentFunction)
  ;[1 1 1] 딱 한줄 가져옴(모션이 1개라서 이게 더 간단)
  (bind _returnvalue (Utilities|GetDataTableRow (Variables|Default|GetDataTable) "Throw")
    (:then
      (Variables|Default|SetMagicData _returnvalue)
      (Effects|Components|ParticleSystem|SetTemplate (Variables|Default|GetAttachParticle) (.attachparticle (Utilities|Array|Get(acopy) (Variables|Default|GetThrowItems) (Variables|Default|GetCurrentItem))))
      (Rendering|SetVisibility (Variables|Default|GetAttachParticle) false false))))

(event EventOnEquipped
  (|CallParentFunction)
  (Rendering|SetVisibility (Variables|Default|GetAttachParticle) true false)
  (bind _asbp_player (Utilities|Casting|CastToBP_Player (CallFunction|GetOwnertoCharacter)))
  (Default|OnCameraSideMode _asbp_player))

(event EventOnUnEquipped
  (|CallParentFunction)
  (Rendering|SetVisibility (Variables|Default|GetAttachParticle) false false)
  (bind _asbp_player (Utilities|Casting|CastToBP_Player (CallFunction|GetOwnertoCharacter)))
  (Default|OffCameraSideMode _asbp_player))

(event EventSpell
  (bind _ascharacter (CallFunction|GetOwnertoCharacter))
  (bind _magicdata (Variables|Default|GetMagicData))
  (bind (_skilltype _montage _playrate _startsection _canmove) (Utilities|Struct|BreakFMagicData _magicdata))
  (|CallParentFunction)
  (Class|IState|SetCanMove(Message) _ascharacter _canmove)
  (Animation|PlayAnimMontage _ascharacter _montage _playrate _startsection) ; 얘 자체에 뭔가 있어서 못움직였다가 움직여짐
)

(event EventEndSpell
  (|CallParentFunction)
  (Default|SetCanMove (CallFunction|GetOwnertoMagic) true))

(fn ConstructionScript
  (|CallParentFunction))

(fn SetCurrentItem
  (params (New%20Item :type BP%20Throw%20Item%20Class%20Reference))
  (bind _throwitems (Variables|Default|GetThrowItems))
  (bind _array_index (Utilities|Array|ForEachLoopwithBreak _throwitems :!label _label)
    (:LoopBody
      (LocalVariables|SetIndex _array_index)
      (if (== New%20Item (.throwitemclass (Utilities|Array|Get(acopy) _throwitems (LocalVariables|GetIndex))))
        (goto _label Break)))
    (:Completed
      (Variables|Default|SetCurrentItem (LocalVariables|GetIndex))
      (Effects|Components|ParticleSystem|SetTemplate (Variables|Default|GetAttachParticle) (.attachparticle (Utilities|Array|Get(acopy) (Variables|Default|GetThrowItems) (Variables|Default|GetCurrentItem)))))))