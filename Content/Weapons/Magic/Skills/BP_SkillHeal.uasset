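; BP_SkillHeal is a magic skill that heals the character casting it.
; On BeginPlay it caches the single "Heal" DataTable row, since the skill has only one motion.
; Spell applies that row's movement setting, plays its montage and immediately adds a hardcoded health amount through the owner's StatusComponent, if valid.
; EndSpell re-enables movement.
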(event EventBeginPlay
  (|CallParentFunction)
  ;[1 1 1] 딱 한줄 가져옴(모션이 1개라서 이게 더 간단)
  (bind _returnvalue (Utilities|GetDataTableRow (Variables|Default|GetDataTable) "Heal")
    (:then
      (Variables|Default|SetMagicData _returnvalue))))

(event EventSpell
  (bind _ascharacter (CallFunction|GetOwnertoCharacter))
  (bind _magicdata (Variables|Default|GetMagicData))
  (bind (_skilltype _montage _playrate _startsection _canmove) (Utilities|Struct|BreakFMagicData _magicdata))
  (bind _returnvalue (Actor|GetComponentbyClass _ascharacter "/Game/Components/StatusComponent.StatusComponent_C"))
  (|CallParentFunction)
  (Default|SetCanMove (CallFunction|GetOwnertoMagic) _canmove)
  (Animation|PlayAnimMontage (CallFunction|GetOwnertoCharacter) _montage _playrate _startsection) ; 얘 자체에 뭔가 있어서 못움직였다가 움직여짐
  (Utilities|IsValid _returnvalue
    (:Is%20Valid
      (Default|IncreaseHealth _returnvalue 2e+01))))

(event EventEndSpell
  (|CallParentFunction)
  (Default|SetCanMove (CallFunction|GetOwnertoMagic) true))

(fn ConstructionScript
  (|CallParentFunction))