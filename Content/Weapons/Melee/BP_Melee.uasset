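; Melee weapon Blueprint that runs data-driven combo and smash attacks for its owning character.
; BeginPlay picks a combo table by owner mesh, then caches combo and smash rows matching MeleeType.
; Attack and Smash buffer input for PlayNextCombo, which plays the next combo montage or a smash keyed by combo and smash counts, using stamina where the owner has it.
; SendDamage filters repeat hits until OffCollision; empty combo and damage-effect hooks are exposed.
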(event Custom|DamageEffect)

(event EventBeginPlay
  ;[1 1 1] 데이터테이블(콤보 몽타쥬) 읽어오기
  (|CallParentFunction)
  (Utilities|FlowControl|Sequence
    (:then_0
      (|ReadOwnerMeshAndSetDataTable))
    (:then_1
      (|ReadMeleeType))
    (:then_2
      (|ReadSmashType))))

(fn ConstructionScript
  (|CallParentFunction))

(fn Attack
  (|CallParentFunction)
  (if (Variables|Combo|GetCanCombo) ; 난 Attack 함수가 왜 Melee에 있지\n왜냐면 난 함수고, 수업은 이벤트니까
    (Variables|Combo|SetCanCombo false)
    (Variables|Combo|SetSucceedCombo true)
    (elif (CallFunction|CanAttack)
      (CallFunction|SetStateAttacking)
      (CallFunction|PlayComboMontage)
      (CallFunction|StartCombo))))

(fn PlayComboMontage
  (bind _melee_datas (Variables|Combo|GetMelee%20Datas))
  (bind _combocount (Variables|Combo|GetComboCount))
  (bind _output (Utilities|Array|Get(acopy) _melee_datas _combocount))
  (bind _ascharacter (Utilities|Casting|CastToCharacter (Components|GetOwner)))
  (if (> (Utilities|Array|Length _melee_datas) _combocount)
    (Animation|PlayAnimMontage _ascharacter (.montage _output) (.playrate _output) (.startsection _output))
    (CallFunction|SetCanMove (.canmove _output))
    (Variables|Default|SetIsSmashing false)))

(fn PlayNextCombo
  (if (Variables|Combo|GetSucceedCombo)
    (if (Variables|Combo|GetSucceedSmash)
      (CallFunction|PlaySmashMontage)
      (Math|Integer|IncrementInt (Variables|Combo|GetSamshCount)
        (:%20%20
          _))
      (else
        (Math|Integer|IncrementInt (Variables|Combo|GetComboCount)
          (:%20%20
            (CallFunction|PlayComboMontage)))))
    (Variables|Combo|SetSucceedCombo false)
    (Variables|Combo|SetSucceedSmash false)
    (Variables|Default|SetIsLastCombo (== (- (Utilities|Array|Length (Variables|Combo|GetMelee%20Datas)) 1) (Variables|Combo|GetComboCount)))))

(fn OnCollision
  (params (FistCollisionType :type EFistCollisionType%20Enum :default "NewEnumerator0") (SmashHitIndex :type Integer))
  (Variables|Combo|SetSmashHitIndex SmashHitIndex))

(fn OffCollision
  (Utilities|Array|Clear (Variables|Default|GetHittedActors)))

(fn SendDamage
  (params (Other%20Actor :type Actor%20Object%20Reference) (Damage :type Float%20%28single-precision%29) (NewParam :type Boolean) (DamageTypeClass :type Damage%20Type%20Class%20Reference))
  (bind _array_element (Utilities|Array|ForEachLoopwithBreak (Variables|Default|GetHittedActors) :!label _label)
    (:LoopBody
      (if (== _array_element Other%20Actor)
        (LocalVariables|SetEverHittedActor true)
        (goto _label Break)))
    (:Completed
      (if (LocalVariables|GetEverHittedActor)
        (return false)
        (else
          (Utilities|Array|Add (Variables|Default|GetHittedActors) Other%20Actor)
          (bind _result (|CallParentFunction Other%20Actor Damage false DamageTypeClass))
          (if _result
            (CallFunction|DamageEffect)
            (return _result)))))))

(fn EndAttack
  ;[1 1 1] 공격 끝
  (|CallParentFunction)
  (CallFunction|SetStateIdling)
  (Variables|Combo|SetComboCount 0)
  (Variables|Combo|SetSamshCount 0)
  (CallFunction|SetCanMove true)
  (Variables|Combo|SetSucceedCombo false)
  (Variables|Default|SetIsLastCombo false)
  (Variables|Combo|SetSucceedSmash false)
  (CallFunction|EndCombo))

(fn StartCombo)

(fn EndCombo)

(fn PlaySmashMontage
  (bind (_statuscomp _isvalid) (CallFunction|GetOwnertoStatusComponent))
  (bind (_statuscomp_2 _isvalid_2) (CallFunction|GetOwnertoStatusComponent))
  (bind _samshcount (Variables|Combo|GetSamshCount))
  (bind _combocount (Variables|Combo|GetComboCount))
  (bind _smashdatas (Variables|Combo|GetSmashDatas))
  (bind _returnvalue (Utilities|String|ToString(Integer) _samshcount))
  (bind _returnvalue_2 (Utilities|String|ToString(Integer) _combocount))
  (bind _returnvalue_3 (Utilities|String|Append _returnvalue_2 "_" _returnvalue))
  (bind _returnvalue_4 (Utilities|String|StringToName _returnvalue_3))
  (bind _value (Utilities|Map|Find _smashdatas _returnvalue_4))
  (bind _ascharacter (Utilities|Casting|CastToCharacter (Components|GetOwner)))
  (if _isvalid
    ;[1 1 1] 스테이터스 Get 구현을 한 개체만 검사 (Enemy는 구현을 안했어)
    (if (>= (Variables|/Game/Components/StatusComponent.StatusComponent_C|GetCurrentStamina _statuscomp) (.needstaminaamount _value))
      (Animation|PlayAnimMontage _ascharacter (.montage _value) (.playrate _value) (.startsection _value) :!label _label)
      (CallFunction|SetCanMove (.canmove _value))
      (Variables|Default|SetIsSmashing true)
      ;[1 1 1] 플레이어만 스태미나 감소
      (if _isvalid_2
        (Default|DecreaseStamina _statuscomp_2 (.needstaminaamount _value))))
    (else
      (goto _label))))

(fn Smash
  (|CallParentFunction)
  (bind _result (Class|IState|IsStateAttacking(Message) (Components|GetOwner)))
  (if _result
    (if (or (Variables|Combo|GetCanCombo) (not (Variables|Combo|GetSucceedSmash))) ; 난 Attack 함수가 왜 Melee에 있지\n왜냐면 난 함수고, 수업은 이벤트니까
      (Variables|Combo|SetCanCombo false)
      (Variables|Combo|SetSucceedCombo true)
      (Variables|Combo|SetSucceedSmash true))))

(fn GetCombatType
  (return (Variables|Default|GetCombatType)))

(fn GetCurrentWeapon
  (return 0))

(fn GetOwnerParticleTrail
  (return 0))

(fn GetSubWeaponWidget
  (return 0))

(fn SetCurrentWeapon
  (params (NewWeapon :type BP%20Weapon%20Object%20Reference))
  (return 0))

(fn WeaponAttach
  (return false))

(fn WeaponDetach
  (return false))

(fn WeaponEquipped
  (return false))

(fn WeaponUnEquipped
  (return false))