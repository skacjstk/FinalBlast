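; BP_GreatSword is a child melee weapon Blueprint for a great sword that deals slash damage during combo attacks.
; Its Capsule hitbox starts disabled and is toggled by the inherited OnCollision and OffCollision events.
; Overlaps query WeaponDamageComponent for combo-based damage and send it to actors whose class differs from the owner's.
; Combo start and end notify that component, with the start marked as the critical hit check.
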(event OnComponentBeginOverlap(Capsule)
  (params (OverlappedComponent :type Primitive%20Component%20Object%20Reference) (OtherActor :type Actor%20Object%20Reference) (OtherComp :type Primitive%20Component%20Object%20Reference) (OtherBodyIndex :type Integer) (bFromSweep :type Boolean) (SweepResult :type Hit%20Result%20Structure%20%28by%20ref%29))
  (bind _returnvalue (Default|GetComboDamage (Variables|Default|GetWeaponDamageComponent) (Variables|Default|GetComboCount) 0 -1))
  (if (!= (Utilities|GetClass OtherActor) (Utilities|GetClass (Components|GetOwner)))
    (CallFunction|SendDamage OtherActor _returnvalue SweepResult "/Game/Components/DamageType/SlashDamage.SlashDamage_C")))

(event EventBeginPlay
  (|CallParentFunction)
  (Collision|SetCollisionEnabled (Variables|Default|GetCapsule) "NoCollision"))

(event EventOnCollision
  (params (FistCollisionType :type EFistCollisionType%20Enum :default "NewEnumerator0") (SmashHitIndex :type Integer))
  (|CallParentFunction "NewEnumerator0" -1)
  (Collision|SetCollisionEnabled (Variables|Default|GetCapsule) "QueryAndPhysics"))

(event EventOffCollision
  (|CallParentFunction)
  (Collision|SetCollisionEnabled (Variables|Default|GetCapsule) "NoCollision"))

(event EventStartCombo
  ;[1 1 1] 치명타 검사
  (|CallParentFunction)
  (Default|StartAttack (Variables|Default|GetWeaponDamageComponent) (Variables|Default|GetComboCount)))

(event EventEndCombo
  ;[1 1 1] 치명타 검사
  (|CallParentFunction)
  (Default|EndAttack (Variables|Default|GetWeaponDamageComponent)))

(fn ConstructionScript)