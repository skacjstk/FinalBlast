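; BP_Katana is a melee katana weapon, a child of a parent weapon Blueprint, that deals slash damage through a blade collider.
; Combo start and end drive its WeaponDamageComponent, which computes overlap damage from combo count, smash count and smash hit index.
; OnCollision and OffCollision toggle the blade between query-only and no collision, starting disabled on BeginPlay.
; Swing particle events begin and end a socket-to-socket weapon trail.
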(event OnComponentBeginOverlap(BladeCollision)
  (params (OverlappedComponent :type Primitive%20Component%20Object%20Reference) (OtherActor :type Actor%20Object%20Reference) (OtherComp :type Primitive%20Component%20Object%20Reference) (OtherBodyIndex :type Integer) (bFromSweep :type Boolean) (SweepResult :type Hit%20Result%20Structure%20%28by%20ref%29))
  (bind _returnvalue (Default|GetComboDamage (Variables|Default|GetWeaponDamageComponent) (Variables|Default|GetComboCount) (Variables|Default|GetSamshCount) (Variables|Default|GetSmashHitIndex)))
  (CallFunction|SendDamage OtherActor _returnvalue false "/Game/Components/DamageType/SlashDamage.SlashDamage_C"))

(event EventOnCollision
  (params (FistCollisionType :type EFistCollisionType%20Enum :default "NewEnumerator0") (SmashHitIndex :type Integer))
  ;[1 1 1] 충돌체 켜고 끄기
  (|CallParentFunction FistCollisionType SmashHitIndex)
  (Collision|SetCollisionEnabled (Variables|Default|GetBladeCollision) "QueryOnly"))

(event EventOffCollision
  ;[1 1 1] 충돌체 켜고 끄기
  (|CallParentFunction)
  (Collision|SetCollisionEnabled (Variables|Default|GetBladeCollision) "NoCollision"))

(event EventBeginPlay
  (|CallParentFunction)
  (CallFunction|OffCollision)
  (Variables|Default|SetIsRotationLock true))

(event EventStartCombo
  (|CallParentFunction)
  (Default|StartAttack (Variables|Default|GetWeaponDamageComponent) (Variables|Default|GetComboCount)))

(event EventPlaySwingParticle
  (params (TrailStart :type Name%20%28by%20ref%29 :default "None") (TrailEnd :type Name%20%28by%20ref%29 :default "None"))
  (Effects|Particles|Trails|BeginTrails (Variables|Default|GetSwingTrail) TrailStart TrailEnd "ETrailWidthMode_FromFirst" 1.0))

(event EventEndCombo
  (|CallParentFunction)
  (Default|EndAttack (Variables|Default|GetWeaponDamageComponent)))

(event EventEndSwingParticle
  (Effects|Particles|Trails|EndTrails (Variables|Default|GetSwingTrail)))

(fn ConstructionScript
  (|CallParentFunction))

(fn GetOwnerParticleTrail
  (return 0))

(fn SetCurrentWeapon
  (params (NewWeapon :type BP%20Weapon%20Object%20Reference))
  (return 0))

(fn GetCurrentWeapon
  (return 0))

(fn GetCombatType
  (return (Variables|Default|GetCombatType)))