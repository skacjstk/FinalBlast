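; BP_Sword is a melee sword weapon that deals combo-based damage to actors its blade collision overlaps.
; Collision starts disabled and is toggled to query-only through OnCollision and OffCollision, which extend the parent's versions.
; On overlap, WeaponDamageComponent supplies damage for the current ComboCount to SendDamage, while StartCombo and EndCombo open and close its attack.
; Swing events begin and end a socket-to-socket trail on SwingTrail.
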(event OnComponentBeginOverlap(SwordCollision)
  (params (OverlappedComponent :type Primitive%20Component%20Object%20Reference) (OtherActor :type Actor%20Object%20Reference) (OtherComp :type Primitive%20Component%20Object%20Reference) (OtherBodyIndex :type Integer) (bFromSweep :type Boolean) (SweepResult :type Hit%20Result%20Structure%20%28by%20ref%29))
  ;[1 1 1] 무기 피해 주기
  (bind _returnvalue (Default|GetComboDamage (Variables|Default|GetWeaponDamageComponent) (Variables|Default|GetComboCount)))
  (CallFunction|SendDamage OtherActor _returnvalue))

(event EventBeginPlay
  (|CallParentFunction)
  (CallFunction|OffCollision))

(event Collision|EventActorBeginOverlap
  (params (OtherActor :type Actor%20Object%20Reference)))

(event EventOnCollision
  (params (FistCollisionType :type EFistCollisionType%20Enum :default "NewEnumerator0"))
  ;[1 1 1] 충돌체 켜고 끄기
  (|CallParentFunction FistCollisionType)
  (Collision|SetCollisionEnabled (Variables|Default|GetSwordCollision) "QueryOnly"))

(event EventPlaySwingParticle
  (params (TrailStart :type Name%20%28by%20ref%29 :default "None") (TrailEnd :type Name%20%28by%20ref%29 :default "None"))
  (Effects|Particles|Trails|BeginTrails (Variables|Default|GetSwingTrail) TrailStart TrailEnd "ETrailWidthMode_FromFirst" 1.0))

(event EventOffCollision
  ;[1 1 1] 충돌체 켜고 끄기
  (|CallParentFunction)
  (Collision|SetCollisionEnabled (Variables|Default|GetSwordCollision) "NoCollision"))

(event EventEndSwingParticle
  (Effects|Particles|Trails|EndTrails (Variables|Default|GetSwingTrail)))

(event EventStartCombo
  ;[1 1 1] 치명타 판단용
  (|CallParentFunction)
  (Default|StartAttack (Variables|Default|GetWeaponDamageComponent)))

(event EventEndCombo
  ;[1 1 1] 치명타 판단용
  (|CallParentFunction)
  (Default|EndAttack (Variables|Default|GetWeaponDamageComponent)))

(fn ConstructionScript)

(fn GetCombatType
  (return (Variables|Default|GetCombatType)))

(fn GetCurrentWeapon
  (return 0))

(fn GetOwnerParticleTrail
  (return 0))

(fn SetCurrentWeapon
  (params (NewWeapon :type BP%20Weapon%20Object%20Reference))
  (return 0))