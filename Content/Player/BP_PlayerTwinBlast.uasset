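; Player character Blueprint for TwinBlast that sets up mesh, animation, montage table and sunglasses, and adds katana equipping.
; BeginPlay hides unused weapon bones and spawns the katana on a holster socket, with functions moving its blade between holster and hand sockets.
; The Sword input branches on combat type to switch weapons through DoOnce-guarded montages.
; Separate completion events update combat state, movement and queued fist or magic switches, while early interruptions trigger failure handling.
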(event EventBeginPlay
  (|CallParentFunction)
  (Utilities|FlowControl|Sequence
    (:then_0
      (|HideUnUsedSocket))
    (:then_2
      (bind _returnvalue (Game|SpawnActorfromClass "/Game/Weapons/Melee/BP_Katana.BP_Katana_C" (Math|Transform|MakeTransform "0, 0, 0") "Undefined" self 0))
      (bind _output_get (Variables|Default|SetKatana _returnvalue))
      (Transformation|AttachComponentToComponent _output_get (Variables|Character|GetMesh) "Holster_Katana" "KeepRelative" "KeepRelative" "KeepRelative" true))))

(event Collision|EventActorBeginOverlap
  (params (OtherActor :type Actor%20Object%20Reference)))

(event EventTick
  (params (DeltaSeconds :type Float%20%28single-precision%29))
  (|CallParentFunction DeltaSeconds) ; 지금 이 노드는 비활성 상태입니다. \n핀을 끌어서 다른 노드를 연결하면 활성화됩니다.
)

(fn ConstructionScript
  (|CallParentFunction)
  (Class|SkeletalMeshComponent|SetAnimClass (Variables|Character|GetMesh) "/Game/Player/AnimBP/ABP_PlayerTwinBlast.ABP_PlayerTwinBlast_C")
  (Variables|Default|SetDataTable "/Game/DataTables/TwinBlast/DT_PlayerTwinBlastMontages.DT_PlayerTwinBlastMontages")
  ;[1 1 1] 안경씌워주기
  (Transformation|AttachComponentToComponent (Variables|Default|GetSM_Cool_Sunglasses2) (Variables|Character|GetMesh) "C_brow_mid" "KeepRelative" "KeepRelative" "KeepRelative" true))

(fn AttachSword
  (bind _katana (Variables|Default|GetKatana))
  (bind _blade (Variables|/Game/Weapons/Melee/BP_Katana.BP_Katana_C|GetBlade _katana))
  (Transformation|DetachFromComponent _blade "KeepRelative" "KeepRelative" "KeepWorld" true)
  (Transformation|AttachComponentToComponent _blade (Variables|Character|GetMesh) "Hand_Katana" "KeepRelative" "KeepRelative" "KeepWorld" true)
  (Variables|Default|SetAttached true))

(fn DetachSword
  (Transformation|AttachComponentToComponent (Variables|/Game/Weapons/Melee/BP_Katana.BP_Katana_C|GetBlade (Variables|Default|GetKatana)) (Variables|Character|GetMesh) "Holster_Katana" "KeepRelative" "KeepRelative" "KeepRelative" true)
  (Variables|Default|SetAttached false))

(fn HandReserveSword
  (Transformation|AttachComponentToComponent (Variables|/Game/Weapons/Melee/BP_Katana.BP_Katana_C|GetBlade (Variables|Default|GetKatana)) (Variables|Character|GetMesh) "Hand_katana_Reverse" "KeepRelative" "KeepRelative" "KeepRelative" true))

(event Custom|EquippedSword
  (bind _charactermovement (Variables|Character|GetCharacterMovement))
  ;[1 1 1] 칼 장착
  (Variables|Default|SetEquippedComplete true)
  (Variables|Default|SetStateType "NewEnumerator0")
  (CallFunction|SetCurrentWeapon (Variables|Default|GetKatana))
  (Variables|Default|SetCombatType "NewEnumerator1")
  (Variables|Default|SetbUseControllerRotationYaw true)
  (Variables|/Script/Engine.CharacterMovementComponent|SetbOrientRotationToMovement (Variables|Character|GetCharacterMovement) false)
  (Variables|Default|SetCanMove true)
  (Variables|/Script/Engine.CharacterMovementComponent|SetMaxWalkSpeed _charactermovement 6e+02)
  (Utilities|FlowControl|DoOnce false) ; enters at Reset
)

(event Custom|UnEquipSword
  ;[1 1 1] 칼 해제
  (Variables|Default|SetStateType "NewEnumerator2")
  (Utilities|FlowControl|DoOnce false :!label _label
    (:Completed
      (Animation|Montage|PlayMontage (Variables|Character|GetMesh) (.Value (Utilities|Map|Find (Variables|Default|GetMontageDatas) (Utilities|Array|Get(acopy) (Variables|Default|GetMontageNames) 3)))
        (:then
          (Variables|/Script/Engine.CharacterMovementComponent|SetMaxWalkSpeed (Variables|Character|GetCharacterMovement) 0.0)
          (Variables|Default|SetEquippedComplete false))
        (:OnInterrupted
          (if (not (Variables|Default|GetEquippedComplete))
            (CallFunction|FailEquipSowrd)
            (CallFunction|WeaponAttach)
            (goto _label Reset)))))))

(event Custom|UnEqippedSword
  ;[1 1 1] 칼 해제
  (Variables|Default|SetEquippedComplete true)
  (Variables|Default|SetStateType "NewEnumerator0")
  (Variables|Default|SetCombatType "NewEnumerator0")
  (Variables|Default|SetbUseControllerRotationYaw false)
  (Variables|/Script/Engine.CharacterMovementComponent|SetbOrientRotationToMovement (Variables|Character|GetCharacterMovement) true)
  (Variables|Default|SetCanMove true)
  (CallFunction|SetCurrentWeapon)
  (Utilities|FlowControl|Sequence
    (:then_0
      (if (Variables|Default|GetChangeFistMode)
        (CallFunction|EquipFist)
        (Variables|Default|SetChangeFistMode false)
        (Utilities|FlowControl|DoOnce false) ; enters at Reset
        (else
          (Variables|/Script/Engine.CharacterMovementComponent|SetMaxWalkSpeed (Variables|Character|GetCharacterMovement) 6e+02)
          (Utilities|FlowControl|DoOnce false) ; enters at Reset
        )))
    (:then_1
      (if (Variables|Default|GetChangeMagicMode)
        (CallFunction|EquipMagic)
        (Variables|Default|SetChangeMagicMode false)))))

(event Custom|EquipSword
  ;[1 1 1] 칼 장착
  (Variables|Default|SetStateType "NewEnumerator1")
  (Utilities|FlowControl|DoOnce false :!label _label
    (:Completed
      (Animation|Montage|PlayMontage (Variables|Character|GetMesh) (.Value (Utilities|Map|Find (Variables|Default|GetMontageDatas) (Utilities|Array|Get(acopy) (Variables|Default|GetMontageNames) 2))) 0.8
        (:then
          (Variables|/Script/Engine.CharacterMovementComponent|SetMaxWalkSpeed (Variables|Character|GetCharacterMovement) 4e+02)
          (Variables|Default|SetEquippedComplete false))
        (:OnInterrupted
          (if (not (Variables|Default|GetEquippedComplete))
            (CallFunction|FailEquipSowrd)
            (CallFunction|WeaponDetach)
            (goto _label Reset)))))))

(event Input|ActionEvents|InputActionSword
  (params (Key :type Key%20Structure))
  ;[1 1 1] 2번 누르면 소드 장착/해제
  (:Pressed
    (bind _result (CallFunction|IsStateIdling))
    (if _result
      (switch Utilities|FlowControl|Switch|SwitchonECombatType (Variables|Default|GetCombatType)
        (:NewEnumerator0
          (CallFunction|EquipSword))
        (:NewEnumerator1
          (bind _asbp_melee (Utilities|Casting|CastToBP_Melee (Variables|Default|GetCurrentWeapon)))
          (switch Utilities|FlowControl|Switch|SwitchonEMeleeType (Variables|/Game/Weapons/Melee/BP_Melee.BP_Melee_C|GetMeleeType _asbp_melee)
            (:NewEnumerator1
              (CallFunction|UnEquipFist)
              (CallFunction|EquipSword))
            (:NewEnumerator4
              (CallFunction|UnEquipSword)
              (Variables|Default|SetChangeFistMode false))))
        (:NewEnumerator2
          (CallFunction|UnEquipMagic)
          (CallFunction|EquipSword))
        (:NewEnumerator3
          (CallFunction|UnEquipRifle))))))